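; Game instance that tracks the overall game state and chosen mode (Single Player, Co-op, Versus) and drives level transitions.
; State-gated events open the matching character select screen or gameplay map, with Co-op and Single Player sharing one map.
; It also quits from the main menu, returns to the menu while removing extra local players, and creates or removes the loading screen widget.
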(event Custom|TriggerLoadingScreen
  (bind _returnvalue (UserInterface|CreateWidget "/Game/Student/UI/LoadingScreen.LoadingScreen_C"))
  (bind _output_get (Variables|Default|SetLoading%20Screen%20Widget _returnvalue))
  (UserInterface|Viewport|AddtoViewport _output_get 0))

(event Custom|ExitGame
  (switch Utilities|FlowControl|Switch|SwitchonMainGameStates (Variables|Default|GetCurrentState)
    (:NewEnumerator1
      (Game|QuitGame 0 "Quit"))))

(event Custom|ReturnToMainMenu
  (switch Utilities|FlowControl|Switch|SwitchonMainGameStates (Variables|Default|GetCurrentState)
    (:NewEnumerator1
      _)
    (:NewEnumerator5
      _)
    (:NewEnumerator2
      _)
    (:NewEnumerator3
      _)
    (:NewEnumerator4
      _))
  (Game|OpenLevel(byName) "MenuScreen")
  (Class|GameplayStatics|RemovePlayer (Game|GetPlayerController 1) false)
  (Class|GameplayStatics|RemovePlayer (Game|GetPlayerController 2) false)
  (Class|GameplayStatics|RemovePlayer (Game|GetPlayerController 3) false))

(event Custom|TriggerLoadingScreenDestruction
  (bind _loading_screen_widget (Variables|Default|GetLoading%20Screen%20Widget))
  (Utilities|IsValid _loading_screen_widget
    (:Is%20Valid
      (Widget|RemovefromParent _loading_screen_widget))))

(event Custom|UpdateGameMode
  (params (GameMode :type GameModes%20Enum :default "NewEnumerator0"))
  (Variables|Default|SetGameMode GameMode))

(event Custom|UpdateMainGameState
  (params (GameState :type MainGameStates%20Enum :default "NewEnumerator0"))
  (Variables|Default|SetCurrentState GameState))

(event Custom|Open%20Character%20Select
  (switch Utilities|FlowControl|Switch|SwitchonMainGameStates (Variables|Default|GetCurrentState)
    (:NewEnumerator1
      (switch Utilities|FlowControl|Switch|SwitchonGameModes (Variables|Default|GetGameMode)
        (:NewEnumerator0
          (Game|OpenLevel(byName) "CharacterSelect"))
        (:NewEnumerator1
          (Game|OpenLevel(byName) "VersusCharacterSelect"))
        (:NewEnumerator2
          (Game|OpenLevel(byName) "SinglePlayerCharacterSelect"))))))

(event Custom|StartLevel
  (switch Utilities|FlowControl|Switch|SwitchonMainGameStates (Variables|Default|GetCurrentState)
    (:NewEnumerator1
      _)
    (:NewEnumerator5
      _))
  (switch Utilities|FlowControl|Switch|SwitchonGameModes (Variables|Default|GetGameMode)
    (:NewEnumerator0
      (Game|OpenLevel(byName) "SinglePlayerMap" :!label _label))
    (:NewEnumerator1
      (Game|OpenLevel(byName) "VersusMap"))
    (:NewEnumerator2
      (goto _label))))

(event EventInit
  (Variables|Default|SetCurrentState "NewEnumerator0"))
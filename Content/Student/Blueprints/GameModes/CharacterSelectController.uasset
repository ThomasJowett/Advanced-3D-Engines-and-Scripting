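; Player controller for the character select screen that lets each local player join and then ready up.
; On begin play it caches the CharacterSelectGameMode and switches input to game and UI.
; Gamepad bottom face button and Space share one handler: the first press reports a join to the game mode by controller ID, the next reports ready.
; Two boolean flags track this progress, so further presses do nothing.
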(event EventBeginPlay
  (bind _ascharacter_select_game_mode (Utilities|Casting|CastToCharacterSelectGameMode (Game|GetGameMode)))
  (Variables|Default|SetGameModeRef _ascharacter_select_game_mode)
  (Input|SetInputModeGameandUI self 0 "DoNotLock" true))

(event Input|GamepadEvents|GamepadFaceButtonBottom
  (params (Key :type Key%20Structure))
  (bind _self self)
  (bind _gamemoderef (Variables|Default|GetGameModeRef))
  (:Pressed
    (if (Variables|Default|GetHasJoined)
      (if (not (Variables|Default|GetIsReady))
        (bind _returnvalue (Class|GameplayStatics|GetPlayerControllerID _self))
        (Default|PlayerReady _gamemoderef _returnvalue)
        (Variables|Default|SetIsReady true))
      (else
        (bind _returnvalue_2 (Class|GameplayStatics|GetPlayerControllerID _self))
        (Default|PlayerJoined _gamemoderef _returnvalue_2)
        (Variables|Default|SetHasJoined true)))))

(event Input|KeyboardEvents|SpaceBar
  (params (Key :type Key%20Structure))
  (bind _self self)
  (bind _gamemoderef (Variables|Default|GetGameModeRef))
  (:Pressed
    (if (Variables|Default|GetHasJoined)
      (if (not (Variables|Default|GetIsReady))
        (bind _returnvalue (Class|GameplayStatics|GetPlayerControllerID _self))
        (Default|PlayerReady _gamemoderef _returnvalue)
        (Variables|Default|SetIsReady true))
      (else
        (bind _returnvalue_2 (Class|GameplayStatics|GetPlayerControllerID _self))
        (Default|PlayerJoined _gamemoderef _returnvalue_2)
        (Variables|Default|SetHasJoined true)))))

(fn ConstructionScript)
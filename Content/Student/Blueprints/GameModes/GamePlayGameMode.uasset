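; Game mode for a local-multiplayer Core defence game that alternates Build and Fight modes.
; On BeginPlay it spawns each player's chosen character and weapon at SpawnPoints, binds death and Core-destroyed events, and shows Core health.
; When all players are ready, EnemyManager starts a wave; placed blocks are destroyed if its path drawing fails.
; GameOver shows a widget, then returns to the main menu after a delay.
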(event Custom|ReturnToMainMenu
  (Utilities|FlowControl|Delay 5.0)
  (Default|ReturntoMainMenu (Variables|Default|GetGameInstanceRef)))

(event EventBeginPlay
  (bind _outactors (Actor|GetAllActorsOfClass "/Game/Student/Blueprints/SpawnPoint.SpawnPoint_C"))
  (Variables|Default|SetPlayerStarts _outactors)
  (bind _outactors_2 (Actor|GetAllActorsOfClass "/Game/Student/Blueprints/Enemies/EnemyManager.EnemyManager_C"))
  (bind _output_get (Variables|Default|SetEnemyManagerRef (Utilities|Array|Get(acopy) _outactors_2)))
  (Utilities|IsValid _output_get
    (:Is%20Valid
      (bind _output_get_2 (Variables|Default|SetGameInstanceRef (.GameInstance (Utilities|GetThisGameInstance))))
      (Default|UpdateMainGameState _output_get_2 "NewEnumerator3")
      (CallFunction|InitialisePlayers)
      (bind _outactors_3 (Actor|GetAllActorsOfClass "/Game/Student/Blueprints/Core.Core_C"))
      (bind _output_get_3 (Variables|Default|SetCore (Utilities|Array|Get(acopy) _outactors_3)))
      (EventDispatchers|BindEventtoCoreDestroyed _output_get_3 (EventDispatchers|CreateEvent :!event GameOver))
      (bind _returnvalue (UserInterface|CreateWidget "/Game/Student/UI/CoreHealth.CoreHealth_C"))
      (UserInterface|Viewport|AddtoViewport _returnvalue 0))
    (:Is%20Not%20Valid
      (Development|PrintString "Error: Enemy Manager not found" true true "(R=1.000000,G=0.000000,B=0.000000,A=1.000000)" 1e+03))))

(event EventPlayerReady
  (CallFunction|PlayerReadyGM))

(event EventBlockPlaced
  (params (LastBlockPlaced :type Actor%20Object%20Reference))
  (CallFunction|BlockPlacedGM))

(fn ConstructionScript)

(fn PlayerReadyGM
  (bind _result (Math|Integer|IncrementInt (Variables|Default|GetPlayersReady))
    (:%20%20
      (if (== _result (Variables|/Game/Student/Blueprints/MyGameInstance.MyGameInstance_C|GetNumberOfPlayers (Variables|Default|GetGameInstanceRef)))
        (CallFunction|ChangeMode "NewEnumerator1")
        (Variables|Default|SetPlayersReady 0)))))

(fn ChangeMode
  (params (NewState :type GamePlayStates%20Enum :default "NewEnumerator0"))
  (bind _output_get (Variables|Default|SetGameplayState NewState))
  (switch Utilities|FlowControl|Switch|SwitchonGamePlayStates _output_get
    (:NewEnumerator0
      (Default|CallWaveEnded))
    (:NewEnumerator1
      (Default|StartWave (Variables|Default|GetEnemyManagerRef)))))

(fn BlockPlacedGM
  (params (Last%20Block%20Placed :type Actor%20Object%20Reference))
  (bind _enemymanagerref (Variables|Default|GetEnemyManagerRef))
  (Utilities|IsValid _enemymanagerref
    (:Is%20Valid
      (bind _can_find_path (Default|DrawPaths _enemymanagerref))
      (if (not _can_find_path)
        (Actor|DestroyActor Last%20Block%20Placed)))))

(fn InitialisePlayers
  (for _index (range 0 (- (Variables|/Game/Student/Blueprints/MyGameInstance.MyGameInstance_C|GetNumberOfPlayers (Variables|Default|GetGameInstanceRef)) 1))
    (CallFunction|SpawnPlayer _index)))

(fn SpawnPlayer
  (params (Player%20Controller%20ID :type Integer))
  (bind _returnvalue (Utilities|Transform))
  (bind _playerstarts (Variables|Default|GetPlayerStarts))
  (bind _output (Utilities|Array|Get(acopy) _playerstarts Player%20Controller%20ID))
  (bind _defaultrootscene (Variables|/Game/Student/Blueprints/SpawnPoint.SpawnPoint_C|GetDefaultRootScene _output))
  (bind _returnvalue_2 (Transformation|GetWorldTransform _defaultrootscene))
  (switch Utilities|FlowControl|Switch|SwitchonCharacters (Utilities|Array|Get(acopy) (Variables|/Game/Student/Blueprints/MyGameInstance.MyGameInstance_C|GetCharactersChosen (Variables|Default|GetGameInstanceRef)) Player%20Controller%20ID)
    (:NewEnumerator0
      (bind _returnvalue_3 (Game|SpawnActorfromClass "/Game/Student/Blueprints/Characters/MyCharacter_Sweet.MyCharacter_Sweet_C" _returnvalue_2 "Undefined" 0 0))
      (Pawn|Possess (Game|GetPlayerController Player%20Controller%20ID) _returnvalue_3)
      (EventDispatchers|BindEventtoOnDeath _returnvalue_3 (EventDispatchers|CreateEvent :!event SpawnPlayer))
      (bind _returnvalue_4 (Game|SpawnActorfromClass "/Game/Student/Blueprints/PlayerWeapons/RocketLauncher.RocketLauncher_C" _returnvalue "Undefined" 0 0))
      (Class|WeaponsInterface|AttachtoPlayer(Message) _returnvalue_4 _returnvalue_3))
    (:NewEnumerator1
      (bind _returnvalue_5 (Game|SpawnActorfromClass "/Game/Student/Blueprints/Characters/MyCharacter_Skye.MyCharacter_Skye_C" _returnvalue_2 "Undefined" 0 0))
      (Pawn|Possess (Game|GetPlayerController Player%20Controller%20ID) _returnvalue_5)
      (EventDispatchers|BindEventtoOnDeath _returnvalue_5 (EventDispatchers|CreateEvent :!event SpawnPlayer))
      (bind _returnvalue_6 (Game|SpawnActorfromClass "/Game/Student/Blueprints/PlayerWeapons/AssaultRifle.AssaultRifle_C" _returnvalue "Undefined" 0 0))
      (Class|WeaponsInterface|AttachtoPlayer(Message) _returnvalue_6 _returnvalue_5))
    (:NewEnumerator3
      (bind _returnvalue_7 (Game|SpawnActorfromClass "/Game/Student/Blueprints/Characters/MyCharacter_SiMo.MyCharacter_SiMo_C" _returnvalue_2 "Undefined" 0 0))
      (Pawn|Possess (Game|GetPlayerController Player%20Controller%20ID) _returnvalue_7)
      (EventDispatchers|BindEventtoOnDeath _returnvalue_7 (EventDispatchers|CreateEvent :!event SpawnPlayer))
      (bind _returnvalue_8 (Game|SpawnActorfromClass "/Game/Student/Blueprints/PlayerWeapons/SniperRifle.SniperRifle_C" _returnvalue "Undefined" 0 0))
      (Class|WeaponsInterface|AttachtoPlayer(Message) _returnvalue_8 _returnvalue_7))
    (:NewEnumerator4
      (bind _returnvalue_9 (Game|SpawnActorfromClass "/Game/Student/Blueprints/Characters/MyCharacter_Haigen.MyCharacter_Haigen_C" _returnvalue_2 "Undefined" 0 0))
      (Pawn|Possess (Game|GetPlayerController Player%20Controller%20ID) _returnvalue_9)
      (EventDispatchers|BindEventtoOnDeath _returnvalue_9 (EventDispatchers|CreateEvent :!event SpawnPlayer))
      (bind _returnvalue_10 (Game|SpawnActorfromClass "/Game/Student/Blueprints/PlayerWeapons/ShotGun.ShotGun_C" _returnvalue "Undefined" 0 0))
      (Class|WeaponsInterface|AttachtoPlayer(Message) _returnvalue_10 _returnvalue_9))))

(fn GameOver
  (Variables|Default|SetGameplayState "NewEnumerator3")
  (bind _returnvalue (UserInterface|CreateWidget "/Game/Student/UI/GameOver.GameOver_C"))
  (UserInterface|Viewport|AddtoViewport _returnvalue 0)
  (CallFunction|ReturntoMainMenu))

(fn GetCurrentMode
  (return (Variables|Default|GetGameplayState)))
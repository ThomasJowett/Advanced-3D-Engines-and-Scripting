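; Game mode for a two-team versus match that alternates build and fight phases around each team's Core.
; BeginPlay gathers spawn points, Cores and EnemyManagers by team, adds Core health widgets and spawns chosen characters, assigning teams by controller ID parity.
; Ready players trigger enemy waves, and both managers finishing returns play to building.
; Block placements that fail path drawing are refunded, and win functions show Game Over before returning to menu.
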(event Custom|ReturnToMainMenu
  ;[1 1 1] Return to main menu after delay
  (Utilities|FlowControl|Delay 5.0)
  (Default|ReturntoMainMenu (Variables|Default|GetGameInstanceRef)))

(event EventBeginPlay
  (bind (_gameinstance _success) (Utilities|GetThisGameInstance))
  (if _success
    (bind _output_get (Variables|Default|SetGameInstanceRef _gameinstance))
    (Default|UpdateMainGameState _output_get "NewEnumerator3")
    ;[1 1 1] Spawn Points Setup
    (bind _outactors (Actor|GetAllActorsOfClass "/Game/Student/Blueprints/SpawnPoint.SpawnPoint_C"))
    (for _array_element _outactors
      (if (== (Variables|/Game/Student/Blueprints/SpawnPoint.SpawnPoint_C|GetTeam _array_element) 1)
        (Utilities|Array|Add (Variables|Default|GetTeam1PlayerStarts) _array_element)
        (else
          (Utilities|Array|Add (Variables|Default|GetTeam2PlayerStarts) _array_element))))
    ;[1 1 1] Core Setup
    (bind _outactors_2 (Actor|GetAllActorsOfClass "/Game/Student/Blueprints/Core.Core_C"))
    (for _array_element_2 _outactors_2
      (if (== (Variables|/Game/Student/Blueprints/Core.Core_C|GetTeam _array_element_2) 1)
        (bind _output_get_2 (Variables|Default|SetTeam1Core _array_element_2))
        (EventDispatchers|BindEventtoCoreDestroyed _output_get_2 (EventDispatchers|CreateEvent :!event Team2Wins))
        (bind _returnvalue (UserInterface|CreateWidget "/Game/Student/UI/CoreHealth.CoreHealth_C" 0 _output_get_2))
        (UserInterface|Viewport|AddtoViewport _returnvalue 0)
        (else
          (bind _output_get_3 (Variables|Default|SetTeam2Core _array_element_2))
          (EventDispatchers|BindEventtoCoreDestroyed _output_get_3 (EventDispatchers|CreateEvent :!event Team1Wins))
          (bind _returnvalue_2 (UserInterface|CreateWidget "/Game/Student/UI/CoreHealth.CoreHealth_C" 0 _output_get_3))
          (Default|MovetoMiddle _returnvalue_2)
          (UserInterface|Viewport|AddtoViewport _returnvalue_2 0))))
    ;[1 1 1] Enemy Manager Setup
    (bind _outactors_3 (Actor|GetAllActorsOfClass "/Game/Student/Blueprints/Enemies/EnemyManager.EnemyManager_C"))
    (for _array_element_3 _outactors_3
      (if (== (Variables|/Game/Student/Blueprints/Enemies/EnemyManager.EnemyManager_C|GetTeam _array_element_3) 1)
        (Variables|Default|SetEnemyManagerTeam1 _array_element_3)
        (else
          (Variables|Default|SetEnemyManagerTeam2 _array_element_3))))
    (CallFunction|InitialisePlayers)
    (else
      (Development|PrintString "Error: Incorrect Game Instance, Please set game instance to MyGameInstance" true true "(R=1.000000,G=0.000000,B=0.000000,A=1.000000)"))))

(event EventPlayerReady
  (CallFunction|PlayerReadyGM))

(event EventAllEnemiesDead
  (bind _result (Math|Integer|IncrementInt (Variables|Default|GetManagersFinished))
    (:%20%20
      (if (== _result 2)
        (CallFunction|ChangeMode "NewEnumerator0")
        (Variables|Default|SetManagersFinished 0)))))

(fn ConstructionScript)

(fn PlayerReadyGM
  (bind _result (Math|Integer|IncrementInt (Variables|Default|GetPlayersReady))
    (:%20%20
      (if (== _result (Variables|/Game/Student/Blueprints/MyGameInstance.MyGameInstance_C|GetNumberOfPlayersTeam1 (Variables|Default|GetGameInstanceRef)))
        (CallFunction|ChangeMode "NewEnumerator1")
        (Variables|Default|SetPlayersReady 0)))))

(fn InitialisePlayers
  (bind _gameinstanceref (Variables|Default|GetGameInstanceRef))
  (bind _numberofplayersteam1 (Variables|/Game/Student/Blueprints/MyGameInstance.MyGameInstance_C|GetNumberOfPlayersTeam1 _gameinstanceref))
  (for _index (range 0 (- _numberofplayersteam1 1))
    (CallFunction|SpawnPlayer _index))
  (for _index_2 (range _numberofplayersteam1 (+ _numberofplayersteam1 (- (Variables|/Game/Student/Blueprints/MyGameInstance.MyGameInstance_C|GetNumberOfPlayersTeam2 _gameinstanceref) 1)))
    (CallFunction|SpawnPlayer _index_2)))

(fn SpawnPlayer
  (params (PlayerControllerID :type Integer))
  (if (== (Math|Integer|%(Integer) PlayerControllerID 2) 0)
    (LocalVariables|SetTeam 1)
    (LocalVariables|SetSpawnPoint (Utilities|Array|Get(acopy) (Variables|Default|GetTeam1PlayerStarts)))
    (else
      (LocalVariables|SetTeam 2)
      (LocalVariables|SetSpawnPoint (Utilities|Array|Get(acopy) (Variables|Default|GetTeam2PlayerStarts)))))
  (switch Utilities|FlowControl|Switch|SwitchonCharacters (Utilities|Array|Get(acopy) (Variables|/Game/Student/Blueprints/MyGameInstance.MyGameInstance_C|GetCharactersChosen (Variables|Default|GetGameInstanceRef)) PlayerControllerID)
    (:NewEnumerator0
      (bind _returnvalue (Game|SpawnActorfromClass "/Game/Student/Blueprints/Characters/MyCharacter_Sweet.MyCharacter_Sweet_C" (Transformation|GetWorldTransform (Variables|/Game/Student/Blueprints/SpawnPoint.SpawnPoint_C|GetDefaultRootScene (LocalVariables|GetSpawnPoint))) "Undefined" 0 0))
      (Pawn|Possess (Game|GetPlayerController PlayerControllerID) _returnvalue)
      (EventDispatchers|BindEventtoOnDeath _returnvalue (EventDispatchers|CreateEvent :!event SpawnPlayer))
      (Class|CharacterInterface|SetTeam(Message) _returnvalue (LocalVariables|GetTeam)))
    (:NewEnumerator1
      (bind _returnvalue_2 (Game|SpawnActorfromClass "/Game/Student/Blueprints/Characters/MyCharacter_Skye.MyCharacter_Skye_C" (Transformation|GetWorldTransform (Variables|/Game/Student/Blueprints/SpawnPoint.SpawnPoint_C|GetDefaultRootScene (LocalVariables|GetSpawnPoint))) "Undefined" 0 0))
      (Pawn|Possess (Game|GetPlayerController PlayerControllerID) _returnvalue_2)
      (EventDispatchers|BindEventtoOnDeath _returnvalue_2 (EventDispatchers|CreateEvent :!event SpawnPlayer))
      (Class|CharacterInterface|SetTeam(Message) _returnvalue_2 (LocalVariables|GetTeam)))
    (:NewEnumerator3
      (bind _returnvalue_3 (Game|SpawnActorfromClass "/Game/Student/Blueprints/Characters/MyCharacter_SiMo.MyCharacter_SiMo_C" (Transformation|GetWorldTransform (Variables|/Game/Student/Blueprints/SpawnPoint.SpawnPoint_C|GetDefaultRootScene (LocalVariables|GetSpawnPoint))) "Undefined" 0 0))
      (Pawn|Possess (Game|GetPlayerController PlayerControllerID) _returnvalue_3)
      (EventDispatchers|BindEventtoOnDeath _returnvalue_3 (EventDispatchers|CreateEvent :!event SpawnPlayer))
      (Class|CharacterInterface|SetTeam(Message) _returnvalue_3 (LocalVariables|GetTeam)))
    (:NewEnumerator4
      (bind _returnvalue_4 (Game|SpawnActorfromClass "/Game/Student/Blueprints/Characters/MyCharacter_Haigen.MyCharacter_Haigen_C" (Transformation|GetWorldTransform (Variables|/Game/Student/Blueprints/SpawnPoint.SpawnPoint_C|GetDefaultRootScene (LocalVariables|GetSpawnPoint))) "Undefined" 0 0))
      (Pawn|Possess (Game|GetPlayerController PlayerControllerID) _returnvalue_4)
      (EventDispatchers|BindEventtoOnDeath _returnvalue_4 (EventDispatchers|CreateEvent :!event SpawnPlayer))
      (Class|CharacterInterface|SetTeam(Message) _returnvalue_4 (LocalVariables|GetTeam)))))

(fn Team1Wins
  (Variables|Default|SetGameplayState "NewEnumerator3")
  (bind _returnvalue (UserInterface|CreateWidget "/Game/Student/UI/GameOver.GameOver_C" 0 "Team 1 Wins"))
  (UserInterface|Viewport|AddtoViewport _returnvalue 0)
  (CallFunction|ReturntoMainMenu))

(fn Team2Wins
  (Variables|Default|SetGameplayState "NewEnumerator3")
  (bind _returnvalue (UserInterface|CreateWidget "/Game/Student/UI/GameOver.GameOver_C" 0 "Team 2 Wins"))
  (UserInterface|Viewport|AddtoViewport _returnvalue 0)
  (CallFunction|ReturntoMainMenu))

(fn BlockPlaced
  (params (LastBlockPlaced :type Actor%20Object%20Reference) (PlacedBy :type Player%20Controller%20Object%20Reference))
  (bind _enemymanagerteam1 (Variables|Default|GetEnemyManagerTeam1))
  (Utilities|IsValid _enemymanagerteam1
    (:Is%20Valid
      (bind _can_find_path (Default|DrawPaths _enemymanagerteam1))
      (if (not _can_find_path)
        (Actor|DestroyActor LastBlockPlaced)
        (bind _buildobjectcomponent (Class|PlayerControllerInterface|GetBuildObjectComponent(Message) PlacedBy))
        (Default|ReturnResources _buildobjectcomponent)))))

(fn ChangeMode
  (params (NewState :type GamePlayStates%20Enum :default "NewEnumerator0"))
  (bind _output_get (Variables|Default|SetGameplayState NewState))
  (switch Utilities|FlowControl|Switch|SwitchonGamePlayStates _output_get
    (:NewEnumerator0
      (Default|CallWaveEnded))
    (:NewEnumerator1
      (Default|StartWave (Variables|Default|GetEnemyManagerTeam1))))
  (return true))

(fn GetCore
  (params (PlayercontrollerID :type Integer))
  (if (== (Math|Integer|%(Integer) PlayercontrollerID 2) 0)
    (return (Variables|Default|GetTeam2Core))
    (else
      (return (Variables|Default|GetTeam1Core)))))

(fn GetCurrentMode
  (return (Variables|Default|GetGamePlayState)))

(fn GetEnemyManager
  (params (PlayerControllerID :type Integer))
  (if (== (Math|Integer|%(Integer) PlayerControllerID 2) 0)
    (return (Variables|Default|GetEnemyManagerTeam2))
    (else
      (return (Variables|Default|GetEnemyManagerTeam1)))))
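; Game mode for the local multiplayer character select screen.
; On BeginPlay it updates the game instance's main game state, creates three additional local players and adds the CharacterSelect widget to the viewport.
; PlayerJoined and PlayerReady events increment counters and print a debug string.
; When all joined players are ready and more than one has joined, it tells the game instance to start the level.
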(event Custom|PlayerJoined
  (params (PlayerController :type Integer))
  (Math|Integer|IncrementInt (Variables|Default|GetPlayersJoined)
    (:%20%20
      (Development|PrintString "Hello"))))

(event Custom|StartGame
  (Default|StartLevel (Variables|Default|GetGameInstanceRef)))

(event Custom|PlayerReady
  (params (Player%20Controller :type Integer))
  (Math|Integer|IncrementInt (Variables|Default|GetPlayersReady)
    (:%20%20
      (Development|PrintString "Hello")
      (if (and (== (Variables|Default|GetPlayersJoined) (Variables|Default|GetPlayersReady)) (> (Variables|Default|GetPlayersJoined) 1))
        (CallFunction|StartGame)))))

(event EventBeginPlay
  (bind _output_get (Variables|Default|SetGameInstanceRef (.GameInstance (Utilities|GetThisGameInstance))))
  (Default|UpdateMainGameState _output_get "NewEnumerator5")
  (Class|GameplayStatics|CreatePlayer 1)
  (Class|GameplayStatics|CreatePlayer 2)
  (Class|GameplayStatics|CreatePlayer 3)
  (bind _returnvalue (UserInterface|CreateWidget "/Game/Student/UI/CharacterSelect.CharacterSelect_C"))
  (UserInterface|Viewport|AddtoViewport _returnvalue 0))

(fn ConstructionScript)
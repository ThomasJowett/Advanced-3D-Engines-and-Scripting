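; Explosive enemy character Blueprint whose only custom logic is an AddAmmo function that supplies it with grenades.
; AddAmmo spawns a GrenadesPickup, adds its ItemInfo to the InventoryComponent, sends the pickup message with the enemy's controller, then calls ReloadMessage.
; The event graph holds only disabled default events, and the construction script just calls its parent.
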(event EventBeginPlay
  (|CallParentFunction))

(event Collision|EventActorBeginOverlap
  (params (OtherActor :type Actor%20Object%20Reference)))

(event EventTick
  (params (DeltaSeconds :type Float%20%28single-precision%29)))

(fn ConstructionScript
  (|CallParentFunction))

(fn AddAmmo
  (bind _returnvalue (Game|SpawnActorfromClass "/Game/Student/Blueprints/Pickups/GrenadesPickup.GrenadesPickup_C" (Math|Transform|MakeTransform "0, 0, 0" "0, 0, 0" "1,1,1") "Undefined" 0 0))
  (Default|AddItem (Variables|Default|GetInventoryComponent) (Variables|/Game/Student/Blueprints/Pickups/BasePickup.BasePickup_C|GetItemInfo _returnvalue))
  (Class|InventoryInterface|PickupItem(Message) _returnvalue (Pawn|GetController) _returnvalue)
  (Class|PlayerInterface|Reload(Message) self)
  (return))
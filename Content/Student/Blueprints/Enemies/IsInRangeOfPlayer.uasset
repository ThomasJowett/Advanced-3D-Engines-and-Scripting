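; Behavior tree node for enemy AI that flags whether the player is close enough to take priority over the Core.
; On each AI tick it reads the Player and Core objects from the blackboard and measures their distances from the controlled pawn.
; It sets the IsInRangeOfPlayer key true only when the player is within a hardcoded radius and no farther away than the Core.
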(event EventReceiveTickAI
  (params (OwnerController :type AI%20Controller%20Object%20Reference) (ControlledPawn :type Pawn%20Object%20Reference) (DeltaSeconds :type Float%20%28single-precision%29))
  (bind _returnvalue (Class|BTFunctionLibrary|GetOwnersBlackboard))
  (bind _returnvalue_2 (Utilities|Name|MakeLiteralName "Player"))
  (bind _returnvalue_3 (AI|Components|Blackboard|GetValueasObject _returnvalue _returnvalue_2))
  (bind _asactor (Utilities|Casting|CastToActor _returnvalue_3))
  (bind _returnvalue_4 (Transformation|GetDistanceTo ControlledPawn _asactor))
  (AI|Components|Blackboard|SetValueasBool _returnvalue (Utilities|Name|MakeLiteralName "IsInRangeOfPlayer") (and (<= _returnvalue_4 5e+02) (<= _returnvalue_4 (Transformation|GetDistanceTo ControlledPawn (.AsActor (Utilities|Casting|CastToActor (AI|Components|Blackboard|GetValueasObject _returnvalue (Utilities|Name|MakeLiteralName "Core")))))))))
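; Enemy wave manager that spawns AI enemies and switches the game mode once the enemy list empties.
; StartWave clears path splines, increments the wave number and spawns that many behavior-tree-driven enemies at random navigable points around random EnemySpawnPoints, binding their destroy events.
; Removing the last enemy changes the mode and redraws each spawn point's spline, stopping at the first failure.
; GenerateEnemies is only a counting loop that spawns nothing.
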(event EventBeginPlay
  (bind _asgame_play_game_mode (Utilities|Casting|CastToGamePlayGameMode (Game|GetGameMode)))
  (Variables|Default|SetGameModeRef _asgame_play_game_mode)
  (bind _outactors (Actor|GetAllActorsOfClass "/Game/Student/Blueprints/Enemies/EnemySpawnPoint.EnemySpawnPoint_C"))
  (Variables|Default|SetSpawnPoints _outactors))

(fn ConstructionScript)

(fn RemoveEnemeyfromArray
  (params (EnemyRef :type Actor%20Object%20Reference))
  (bind _enemies (Variables|Default|GetEnemies))
  (Utilities|Array|RemoveItem _enemies EnemyRef)
  (if (== (Utilities|Array|Length _enemies) 0)
    (Default|ChangeMode (Variables|Default|GetGameModeRef) "NewEnumerator0")
    (CallFunction|DrawPaths)))

(fn StartWave
  (bind _spawnpoints (Variables|Default|GetSpawnPoints))
  (CallFunction|DeletePaths)
  (bind _result (Math|Integer|IncrementInt (Variables|Default|GetWaveNumber))
    (:%20%20
      (for _index (range 1 _result)
        (bind _returnvalue (AI|SpawnAIFromClass "/Game/Student/Blueprints/Enemies/EnemyCharacter.EnemyCharacter_C" "/Game/Student/Blueprints/Enemies/AIBT.AIBT" (.RandomLocation (Class|NavigationSystem|GetRandomPointinNavigableRadius (Transformation|GetActorLocation (Utilities|Array|Get(acopy) _spawnpoints (Math|Random|RandomIntegerinRange 0 (- (Utilities|Array|Length _spawnpoints) 1)))) 3e+02)) (Utilities|GetRandomRotation) false))
        (Utilities|IsValid _returnvalue
          (:Is%20Valid
            (Utilities|Array|Add (Variables|Default|GetEnemies) _returnvalue)
            (Game|BindEventtoOnDestroyed _returnvalue (EventDispatchers|CreateEvent :!event RemoveEnemeyfromArray))))))))

(fn DrawPaths
  (for _array_element (Variables|Default|GetSpawnPoints)
    (bind _can_find_path (Default|DrawSpline _array_element))
    (if (not _can_find_path)
      (return false)))
  (return true))

(fn DeletePaths
  (for _array_element (Variables|Default|GetSpawnPoints)
    (Default|DeleteSpline _array_element)))

(fn GenerateEnemies
  (if (<= (LocalVariables|GetIterator) (Variables|Default|GetWaveNumber)) :!label _label
    (Utilities|FlowControl|Sequence
      (:then_0
        (Math|Integer|IncrementInt (LocalVariables|GetIterator)))
      (:then_1
        (goto _label)))
    (else
      (return))))
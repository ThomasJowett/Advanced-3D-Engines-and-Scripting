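; Enemy spawn point that displays the navigation route from itself to the Core's attack location as a raised spline mesh path.
; On BeginPlay, DrawSpline runs a synchronous navmesh query and returns false for missing, partial or too-short paths.
; For complete paths it destroys old segments, feeds path points into PrimarySpline and builds non-colliding mesh segments between them.
; An older construction-script version remains disconnected.
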(event EventBeginPlay
  (CallFunction|DrawSpline))

(fn ConstructionScript)

(fn DrawSpline
  (bind _spline_hieght (Variables|Default|GetSpline%20Hieght))
  (bind _primaryspline (Variables|Default|GetPrimarySpline))
  (bind _primaryspline_2 (Variables|Default|GetPrimarySpline))
  (bind _returnvalue (Class|NavigationSystem|FindPathtoLocationSynchronously (Transformation|GetWorldLocation (Variables|Default|GetDefaultSceneRoot)) (Transformation|GetWorldLocation (Variables|/Game/Student/Blueprints/Core.Core_C|GetAttackLocation (Variables|Default|GetCore)))))
  (Utilities|IsValid _returnvalue
    (:Is%20Valid
      (if (Class|NavigationPath|IsPartial _returnvalue)
        _
        (else
          (CallFunction|DeleteSpline)
          (Variables|Default|SetPath%20array (Variables|/Script/Engine.NavigationPath|GetPathPoints _returnvalue))
          (if (> (Utilities|Array|Length (Variables|Default|GetPath%20array)) 1)
            (Spline|SetSplinePoints _primaryspline (Variables|Default|GetPath%20array) "World" true)
            (for _index (range 0 (- (Spline|GetNumberOfSplinePoints _primaryspline) 2))
              (bind _returnvalue_2 (AddComponent|AddSplineMeshComponent false))
              (Collision|SetCollisionEnabled _returnvalue_2 "NoCollision")
              (Components|StaticMesh|SetStaticMesh _returnvalue_2 (Variables|Default|GetSplineMesh))
              (Rendering|Material|SetMaterial _returnvalue_2 0 (Variables|Default|GetSplineMaterial))
              (Utilities|Array|Add (Variables|Default|GetSplineMeshComponents) _returnvalue_2)
              (SplineMesh|SetStartandEnd _returnvalue_2 (Math|Vector|MakeVector (.X (Math|Vector|BreakVector (.Location (Spline|GetLocationandTangentatSplinePoint _primaryspline_2 _index "Local")))) (.Y (Math|Vector|BreakVector (.Location (Spline|GetLocationandTangentatSplinePoint _primaryspline_2 _index "Local")))) (+ (.Z (Math|Vector|BreakVector (.Location (Spline|GetLocationandTangentatSplinePoint _primaryspline_2 _index "Local")))) _spline_hieght)) (Math|Vector|MakeVector (.X (Math|Vector|BreakVector (.Tangent (Spline|GetLocationandTangentatSplinePoint _primaryspline_2 _index "Local")))) (.Y (Math|Vector|BreakVector (.Tangent (Spline|GetLocationandTangentatSplinePoint _primaryspline_2 _index "Local")))) (+ (.Z (Math|Vector|BreakVector (.Tangent (Spline|GetLocationandTangentatSplinePoint _primaryspline_2 _index "Local")))) _spline_hieght)) (Math|Vector|MakeVector (.X (Math|Vector|BreakVector (.Location (Spline|GetLocationandTangentatSplinePoint _primaryspline_2 (+ _index 1) "Local")))) (.Y (Math|Vector|BreakVector (.Location (Spline|GetLocationandTangentatSplinePoint _primaryspline_2 (+ _index 1) "Local")))) (+ (.Z (Math|Vector|BreakVector (.Location (Spline|GetLocationandTangentatSplinePoint _primaryspline_2 (+ _index 1) "Local")))) _spline_hieght)) (Math|Vector|MakeVector (.X (Math|Vector|BreakVector (.Tangent (Spline|GetLocationandTangentatSplinePoint _primaryspline_2 (+ _index 1) "Local")))) (.Y (Math|Vector|BreakVector (.Tangent (Spline|GetLocationandTangentatSplinePoint _primaryspline_2 (+ _index 1) "Local")))) (+ (.Z (Math|Vector|BreakVector (.Tangent (Spline|GetLocationandTangentatSplinePoint _primaryspline_2 (+ _index 1) "Local")))) _spline_hieght)) true :!class /Script/Engine.SplineMeshComponent))
            (return true)
            (else
              _)))))
    (:Is%20Not%20Valid
      _))
  (return false))

(fn DeleteSpline
  (for _array_element (Variables|Default|GetSplineMeshComponents)
    (Utilities|IsValid _array_element
      (:Is%20Valid
        (Components|DestroyComponent _array_element)))))
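; Enemy character that spawns with a shotgun, fires it on command, and drops random pickups when killed.
; BeginPlay rolls up to five random loot types and attaches a collision-free shotgun with a large ammo load.
; Attack fires the equipped weapon, gated by its rate of fire, and SetTeam passes the team's Core to the AI controller.
; Death notifies the game mode, scatters the loot nearby, then destroys the actor after a delay.
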(event Custom|DelayedDestroy
  (Utilities|FlowControl|Delay 2.0)
  (Actor|DestroyActor))

(event EventBeginPlay
  (|CallParentFunction)
  (CallFunction|GenerateLoot)
  (bind _returnvalue (Game|SpawnActorfromClass "/Game/Student/Blueprints/PlayerWeapons/ShotGun.ShotGun_C" (Math|Transform|MakeTransform "0, 0, 0" "0, 0, 0" "1,1,1") "Undefined" 0 0))
  (Class|WeaponsInterface|AttachtoPlayer(Message) _returnvalue self)
  (Variables|/Game/Student/Blueprints/PlayerWeapons/BasePlayerWeapon.BasePlayerWeapon_C|SetCurrentAmmoLoaded _returnvalue 100)
  (Collision|SetActorEnableCollision _returnvalue false))

(event EventSetTeam
  (params (Team :type Integer))
  (bind _asenemy_aicontroller (Utilities|Casting|CastToEnemyAIController (Pawn|GetController)))
  (bind _outactors (Actor|GetAllActorsOfClass "/Game/Student/Blueprints/Core.Core_C"))
  (Default|SetCore _asenemy_aicontroller (Utilities|Array|Get(acopy) _outactors Team)))

(event EventAttack
  (bind _inventorycomponent (Variables|Default|GetInventoryComponent))
  (bind _equippedweapon (Variables|/Game/Student/Blueprints/Inventory/InventoryComponent.InventoryComponent_C|GetEquippedWeapon _inventorycomponent))
  (if (Variables|Default|GetCanAttack)
    (Variables|Default|SetCanAttack false)
    (Class|WeaponsInterface|FireWeapon(Message) _equippedweapon (Variables|Default|GetThirdPersonCamera))
    (Utilities|IsValid _equippedweapon
      (:Is%20Valid
        (Utilities|FlowControl|Delay (Variables|/Game/Student/Blueprints/BaseWeapon.BaseWeapon_C|GetRateOfFire _equippedweapon))
        (Variables|Default|SetCanAttack true)))))

(fn ConstructionScript
  (|CallParentFunction))

(fn DropLoot
  (bind _self self)
  (bind _location (Utilities|GetLocationAroundActor _self 64.0 96.0))
  (for _array_element (Variables|Default|GetResourcesToDrop)
    (switch Utilities|FlowControl|Switch|SwitchonPickUpTypes _array_element
      (:NewEnumerator0
        (Game|SpawnActorfromClass "/Game/Student/Blueprints/Pickups/GrenadesPickup.GrenadesPickup_C" _location "Undefined" 0 0))
      (:NewEnumerator1
        (Game|SpawnActorfromClass "/Game/Student/Blueprints/Pickups/BulletsPickup.BulletsPickup_C" _location "Undefined" 0 0))
      (:NewEnumerator2
        (Game|SpawnActorfromClass "/Game/Student/Blueprints/Pickups/SpringsPickup.SpringsPickup_C" _location "Undefined" 0 0))
      (:NewEnumerator3
        (Game|SpawnActorfromClass "/Game/Student/Blueprints/Pickups/MetalSheetsPickup.MetalSheetsPickup_C" _location "Undefined" 0 0))
      (:NewEnumerator4
        (Game|SpawnActorfromClass "/Game/Student/Blueprints/Pickups/PipesPickup.PipesPickup_C" _location "Undefined" 0 0))
      (:NewEnumerator5
        (Game|SpawnActorfromClass "/Game/Student/Blueprints/Pickups/HealthPickup.HealthPickup_C" _location "Undefined" 0 0)))))

(fn GenerateLoot
  (for _index (range 0 (Math|Random|RandomIntegerinRange 0 5))
    (Utilities|Array|Add (Variables|Default|GetResourcesToDrop) (Utilities|Enum|ByteToEnumPickUpTypes (Math|Conversions|ToByte(Integer) (Math|Random|RandomIntegerinRange 0 (- (|GetNumEnumEntries) 1)))))))

(fn Die
  (bind _newdeath (|CallParentFunction))
  (if _newdeath
    (Class|EnemyInterface|Died(Message) (Game|GetGameMode) self)
    (CallFunction|DropLoot)
    (CallFunction|DelayedDestroy)
    (return true)
    (else
      (return false))))
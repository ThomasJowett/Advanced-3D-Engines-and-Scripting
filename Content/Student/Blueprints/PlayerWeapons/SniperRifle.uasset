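; SniperRifle is a player weapon Blueprint that handles scoping in and out.
; Scoping in narrows the supplied camera's field of view and adds a Scope widget to the owning player's screen.
; Scoping out restores the wider view and removes the widget.
; The controlled pawn's OnDestroyed event is also bound to that removal, so the scope overlay clears if the pawn is destroyed while scoped.
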(event Custom|RemoveWidget
  (params (DestroyedActor :type Actor%20Object%20Reference))
  (bind _scopeui (Variables|Default|GetScopeUI))
  (Utilities|IsValid _scopeui
    (:Is%20Valid
      (Widget|RemovefromParent _scopeui))))

(event EventBeginPlay
  (|CallParentFunction))

(event Collision|EventActorBeginOverlap
  (params (OtherActor :type Actor%20Object%20Reference))
  (|CallParentFunction OtherActor))

(event EventTick
  (params (DeltaSeconds :type Float%20%28single-precision%29))
  (|CallParentFunction DeltaSeconds))

(event EventScopedin
  (params (Camera :type Camera%20Component%20Object%20Reference) (PlayerController :type Player%20Controller%20Object%20Reference))
  (Variables|/Script/Engine.CameraComponent|SetFieldOfView Camera 3e+01)
  (bind _returnvalue (UserInterface|CreateWidget "/Game/Student/UI/Scope.Scope_C" PlayerController))
  (UserInterface|Viewport|AddtoPlayerScreen _returnvalue)
  (Variables|Default|SetScopeUI _returnvalue)
  (bind _controlledpawn (Class|PlayerControllerInterface|GetControlledPawn(Message) PlayerController))
  (Game|BindEventtoOnDestroyed _controlledpawn (delegate Custom|RemoveWidget)))

(event EventUnScopedin
  (params (Camera :type Camera%20Component%20Object%20Reference))
  (Variables|/Script/Engine.CameraComponent|SetFieldOfView Camera 9e+01)
  (CallFunction|RemoveWidget))

(fn ConstructionScript
  (|CallParentFunction))
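; ShotGun is a player weapon Blueprint that overrides FireWeapon to fire a hitscan pellet spread.
; When the parent FireWeapon succeeds, it loops Visibility line traces from just ahead of the camera, randomly rotating each distant end point in pitch and yaw.
; Each trace applies point damage from ItemInfo and spawns an emitter at the result location, without checking for a hit.
; Debug trace lines stay drawn for the RateOfFire duration.
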(event EventBeginPlay
  (|CallParentFunction))

(event Collision|EventActorBeginOverlap
  (params (OtherActor :type Actor%20Object%20Reference))
  (|CallParentFunction OtherActor))

(event EventTick
  (params (DeltaSeconds :type Float%20%28single-precision%29))
  (|CallParentFunction DeltaSeconds))

(fn ConstructionScript
  (|CallParentFunction))

(fn FireWeapon
  (params (Camera :type Camera%20Component%20Object%20Reference))
  (bind _returnvalue (Math|Vector|GetForwardVector Camera))
  (bind _returnvalue_2 (Transformation|GetWorldLocation Camera))
  (bind _returnvalue_3 (* _returnvalue 2e+14))
  (bind _hasfired (|CallParentFunction Camera))
  (if _hasfired
    (for _index (range 0 20)
      (bind _outhit (Collision|LineTraceByChannel (+ (* (Math|Vector|Normalize _returnvalue) 1e+02) _returnvalue_2) (Math|Vector|RotateVector (+ _returnvalue_2 _returnvalue_3) (Math|Rotator|MakeRotator 0.0 (Math|Random|RandomFloatinRange -2.5 2.5) (Math|Random|RandomFloatinRange -2.5 2.5))) "TraceTypeQuery1" false (Utilities|Array|MakeArray 0 self) "ForDuration" true "(R=1.000000,G=0.000000,B=0.000000,A=1.000000)" "(R=0.000000,G=1.000000,B=0.000000,A=1.000000)" (Variables|Default|GetRateOfFire)))
      (Game|Damage|ApplyPointDamage (.HitActor (Collision|BreakHitResult _outhit)) (Math|Conversions|ToFloat(Integer) (.Damage (Utilities|Struct|BreakInventoryItem (Variables|Default|GetItemInfo)))) _returnvalue_3 _outhit 0 self "/Engine/EngineDamageTypes/DmgTypeBP_Environmental.DmgTypeBP_Environmental_C")
      (Effects|SpawnEmitteratLocation 0 (.Location (Collision|BreakHitResult _outhit))))
    (return true)
    (else
      (return false))))
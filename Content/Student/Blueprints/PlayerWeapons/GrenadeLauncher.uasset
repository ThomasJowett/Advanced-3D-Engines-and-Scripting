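; Grenade launcher player weapon that fires exploding projectiles.
; It overrides FireWeapon, deferring to the parent implementation to decide whether a shot is allowed.
; When the parent succeeds, it spawns an ExplodingProjectile at the ProjectileSpawnArrow transform and returns true, otherwise false.
; BeginPlay and construction only call the parent, and Tick and overlap events are disabled.
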(event EventBeginPlay
  ;[0.9844 1 0.9688] Event Beginplay
  (|CallParentFunction))

(event Collision|EventActorBeginOverlap
  (params (OtherActor :type Actor%20Object%20Reference))
  (|CallParentFunction OtherActor))

(event EventTick
  (params (DeltaSeconds :type Float%20%28single-precision%29))
  (|CallParentFunction DeltaSeconds))

(fn ConstructionScript
  (|CallParentFunction))

(fn FireWeapon
  (params (Camera :type Camera%20Component%20Object%20Reference))
  (bind _hasfired (|CallParentFunction Camera))
  (if _hasfired
    (Game|SpawnActorfromClass "/Game/Student/Blueprints/Projectiles/ExplodingProjectile.ExplodingProjectile_C" (Transformation|GetWorldTransform (Variables|Default|GetProjectile%20Spawn%20Arrow)) "Undefined" 0 0)
    (return true)
    (else
      (return false))))
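; Rocket launcher player weapon that fires a RocketProjectile toward whatever the camera is aimed at.
; FireWeapon defers to the parent implementation first and returns false if that refuses the shot.
; It then runs a long visibility trace from just ahead of the camera, turns ProjectileSpawnArrow toward any hit point and spawns the rocket from the arrow's transform.
; On a miss the arrow keeps its current rotation.
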(event EventBeginPlay
  (|CallParentFunction))

(event Collision|EventActorBeginOverlap
  (params (OtherActor :type Actor%20Object%20Reference))
  (|CallParentFunction OtherActor))

(event EventTick
  (params (DeltaSeconds :type Float%20%28single-precision%29))
  (|CallParentFunction DeltaSeconds))

(fn ConstructionScript
  (|CallParentFunction))

(fn FireWeapon
  (params (Camera :type Camera%20Component%20Object%20Reference))
  (bind _returnvalue (Math|Vector|GetForwardVector Camera))
  (bind _returnvalue_2 (Transformation|GetWorldLocation Camera))
  (bind _projectile_spawn_arrow (Variables|Default|GetProjectile%20Spawn%20Arrow))
  (bind _hasfired (|CallParentFunction Camera))
  (if _hasfired
    (bind (_outhit _returnvalue_3) (Collision|LineTraceByChannel (+ (* (Math|Vector|Normalize _returnvalue) 1e+02) _returnvalue_2) (+ _returnvalue_2 (* _returnvalue 2e+04)) "TraceTypeQuery1" false (Utilities|Array|MakeArray 0 self) "None"))
    (if _returnvalue_3
      (Transformation|SetWorldRotation _projectile_spawn_arrow (Math|Rotator|FindLookatRotation (Transformation|GetWorldLocation _projectile_spawn_arrow) (.Location (Collision|BreakHitResult _outhit))) false false))
    (Game|SpawnActorfromClass "/Game/Student/Blueprints/Projectiles/RocketProjectile.RocketProjectile_C" (Transformation|GetWorldTransform (Variables|Default|GetProjectile%20Spawn%20Arrow)) "Undefined" 0 0)
    (return true)
    (else
      (return false))))
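; Base player weapon Blueprint that can be picked up, attached to the right hand or back holster, fired and reloaded.
; Interact hands unattached weapons to the inventory component, and highlighting uses custom depth with item rarity as the stencil value.
; FireWeapon spends ammo and calls the parent, with a timer limiting fire rate and a gate re-firing automatic weapons until StopFiring.
; ReloadWeapon draws ammo from the player's inventory.
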(event Custom|ResetCanFire
  ;[1 1 1] Resetting the time so that the player can't rapid fire shoot single fire weapons
  (Variables|Default|SetCanFire true)
  (if (Variables|Default|GetIsAutomaticWeapon)
    (Utilities|FlowControl|Gate true
      (:Exit
        (CallFunction|FireWeapon (Variables|Default|GetCameraRef))))))

(event Custom|OpenGate
  ;[1 1 1] Resetting the time so that the player can't rapid fire shoot single fire weapons
  (Utilities|FlowControl|Gate true) ; enters at Open
)

(event EventBeginPlay
  (|CallParentFunction)
  (Rendering|SetCustomDepthStencilValue (Variables|Default|GetStaticMesh) (Math|Conversions|ToInteger(Byte) (.Rarity (Utilities|Struct|BreakInventoryItem (Variables|Default|GetItemInfo))))))

(event Collision|EventActorBeginOverlap
  (params (OtherActor :type Actor%20Object%20Reference))
  (|CallParentFunction OtherActor))

(event EventInteract
  (params (Interacted%20By :type Player%20Controller%20Object%20Reference))
  ;[1 1 1] Interact
  (if (not (Variables|Default|GetIsAttached))
    (bind _inventorycomponent (Class|CharacterInterface|ReturnInventoryComponent(Message) (Pawn|GetControlledPawn Interacted%20By)))
    (Default|PickupWeapon _inventorycomponent self)))

(event EventStartOutline
  ;[1 1 1] Outline
  (if (not (Variables|Default|GetIsAttached))
    (Rendering|SetRenderCustomDepth (Variables|Default|GetStaticMesh) true)))

(event EventTick
  (params (DeltaSeconds :type Float%20%28single-precision%29))
  (|CallParentFunction DeltaSeconds))

(event EventStopFiring
  ;[1 1 1] Resetting the time so that the player can't rapid fire shoot single fire weapons
  (Utilities|FlowControl|Gate true) ; enters at Close
)

(event EventPickUpWeapon)

(event EventEndOutLine
  ;[1 1 1] Outline
  (Rendering|SetRenderCustomDepth (Variables|Default|GetStaticMesh) false))

(event EventAttachtoPlayer
  (params (Character :type Character%20Object%20Reference))
  ;[1 1 1] Attaching to player
  (CallFunction|AttachtoPlayerHand Character))

(event EventAttachtoPlayerBack
  (params (Character :type Character%20Object%20Reference))
  ;[1 1 1] Attaching to player
  (CallFunction|AttachtoPlayerBack Character))

(fn ConstructionScript
  (|CallParentFunction))

(fn AttachtoPlayerHand
  (params (Character :type Character%20Object%20Reference))
  (bind _staticmesh (Variables|Default|GetStaticMesh))
  (bind _inventorycomponent (Class|CharacterInterface|ReturnInventoryComponent(Message) Character))
  (Transformation|AttachComponentToComponent (Variables|Default|GetStaticMesh) (Variables|/Script/Engine.Character|GetMesh Character) "RightHandSocket_0" "SnapToTarget" "SnapToTarget" "SnapToTarget" true)
  (Utilities|IsValid _inventorycomponent
    (:Is%20Valid
      (Variables|/Game/Student/Blueprints/Inventory/InventoryComponent.InventoryComponent_C|SetEquippedWeapon _inventorycomponent self))
    (:Is%20Not%20Valid
      _))
  (Variables|Default|SetIsAttached true)
  (Physics|SetEnableGravity _staticmesh false)
  (Physics|SetSimulatePhysics _staticmesh false))

(fn AttachtoPlayerBack
  (params (Character :type Character%20Object%20Reference))
  (bind _staticmesh (Variables|Default|GetStaticMesh))
  (bind _inventorycomponent (Class|CharacterInterface|ReturnInventoryComponent(Message) Character))
  (Transformation|AttachComponentToComponent (Variables|Default|GetStaticMesh) (Variables|/Script/Engine.Character|GetMesh Character) "RightBackHolsterSocket" "SnapToTarget" "SnapToTarget" "SnapToTarget" true)
  (Variables|/Game/Student/Blueprints/Inventory/InventoryComponent.InventoryComponent_C|SetBackWeapon _inventorycomponent self)
  (Variables|Default|SetIsAttached true)
  (Physics|SetEnableGravity _staticmesh false)
  (Physics|SetSimulatePhysics _staticmesh false))

(fn ReloadWeapon
  (params (PlayersInventory :type Inventory%20Component%20Object%20Reference))
  (bind (_amount _arrayindex) (Default|GetAmountOfAmmo PlayersInventory (.AmmoType (Utilities|Struct|BreakInventoryItem (Variables|Default|GetItemInfo)))))
  (Variables|Default|SetPlayersAmmo _amount)
  (if (and (< (Variables|Default|GetCurrentAmmoLoaded) (Variables|Default|GetClipSize)) (> (Variables|Default|GetPlayersAmmo) 0))
    (if (>= (Variables|Default|GetClipSize) (Variables|Default|GetPlayersAmmo))
      (bind _output_get (Variables|Default|SetCurrentAmmoLoaded (Variables|Default|GetPlayersAmmo)))
      (bind _success (Default|RemoveItem PlayersInventory (Utilities|Array|Get(acopy) (Variables|/Game/Student/Blueprints/Inventory/InventoryComponent.InventoryComponent_C|GetInventory PlayersInventory) _arrayindex) _output_get))
      (return _success)
      (else
        (bind _output_get_2 (Variables|Default|SetCurrentAmmoLoaded (Variables|Default|GetClipSize)))
        (bind _success_2 (Default|RemoveItem PlayersInventory (Utilities|Array|Get(acopy) (Variables|/Game/Student/Blueprints/Inventory/InventoryComponent.InventoryComponent_C|GetInventory PlayersInventory) _arrayindex) _output_get_2))
        (return _success_2)))
    (else
      (return false))))

(fn FireWeapon
  (params (Camera :type Camera%20Component%20Object%20Reference))
  (CallFunction|OpenGate)
  (Variables|Default|SetCameraRef Camera)
  (if (and (> (Variables|Default|GetCurrentAmmoLoaded) 0) (Variables|Default|GetCanFire))
    (Variables|Default|SetCanFire false)
    (Math|Integer|DecrementInt (Variables|Default|GetCurrentAmmoLoaded)
      (:%20%20
        (Utilities|Time|SetTimerbyFunctionName 0 "ResetCanFire" (Variables|Default|GetRateOfFire))
        (bind _hasfired (|CallParentFunction 0))
        (return _hasfired)))
    (else
      (return false))))
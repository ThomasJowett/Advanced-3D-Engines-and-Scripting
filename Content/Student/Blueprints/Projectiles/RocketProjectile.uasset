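; RocketProjectile is a projectile Blueprint for a rocket that trails sparks in flight and explodes when it hits something.
; BeginPlay attaches the P_Sparks particle emitter to the static mesh, and that mesh's hit event calls Explode, which is not defined in this graph.
; Each Tick sets the actor's pitch from its velocity direction while keeping roll and yaw, so the rocket tips along its flight path.
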(event OnComponentHit(StaticMesh)
  (params (HitComponent :type Primitive%20Component%20Object%20Reference) (OtherActor :type Actor%20Object%20Reference) (OtherComp :type Primitive%20Component%20Object%20Reference) (NormalImpulse :type Vector :default "0, 0, 0") (Hit :type Hit%20Result%20Structure%20%28by%20ref%29))
  (CallFunction|Explode))

(event EventBeginPlay
  (Effects|SpawnEmitterAttached "/Game/StarterContent/Particles/P_Sparks.P_Sparks" (Variables|Default|GetStaticMesh) "None"))

(event Collision|EventActorBeginOverlap
  (params (OtherActor :type Actor%20Object%20Reference))
  (|CallParentFunction OtherActor))

(event EventTick
  (params (DeltaSeconds :type Float%20%28single-precision%29))
  (bind _returnvalue (Transformation|GetActorRotation))
  (Transformation|SetActorRotation (Math|Rotator|MakeRotator (.roll _returnvalue) (.pitch (Math|Rotator|MakeRotfromX (Transformation|GetVelocity))) (.yaw _returnvalue))))

(fn ConstructionScript
  (|CallParentFunction))
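; ExplodingProjectile is a projectile that explodes on a timer rather than on contact.
; On BeginPlay it waits for FuseTime, then calls Explode.
; Explode spawns an Explosion actor at the static mesh, applies environmental radial damage from that point using the DamageRadius sphere component's radius, and destroys itself.
; Overlap and Tick events are disabled, so the fuse is the only trigger in this Blueprint.
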(event EventBeginPlay
  (|CallParentFunction)
  (Utilities|FlowControl|Delay (Variables|Default|GetFuse%20Time))
  (CallFunction|Explode))

(event Collision|EventActorBeginOverlap
  (params (OtherActor :type Actor%20Object%20Reference))
  (|CallParentFunction OtherActor))

(event EventTick
  (params (DeltaSeconds :type Float%20%28single-precision%29))
  (|CallParentFunction DeltaSeconds))

(fn ConstructionScript
  (|CallParentFunction))

(fn Explode
  (Game|SpawnActorfromClass "/Game/Student/Blueprints/Projectiles/Explosion.Explosion_C" (Transformation|GetWorldTransform (Variables|Default|GetStaticMesh)) "Undefined" 0 0)
  (Game|Damage|ApplyRadialDamage 5e+01 (Transformation|GetWorldLocation (Variables|Default|GetStaticMesh)) (Variables|/Script/Engine.SphereComponent|GetSphereRadius (Variables|Default|GetDamageRadius)) "/Engine/EngineDamageTypes/DmgTypeBP_Environmental.DmgTypeBP_Environmental_C" 0 self 0 false "ECC_WorldDynamic")
  (Actor|DestroyActor))
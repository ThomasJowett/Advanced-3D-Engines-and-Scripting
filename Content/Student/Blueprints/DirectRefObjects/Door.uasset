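; Door actor Blueprint that swings its static mesh open and closed on request through OpenDoor and CloseDoor events.
; BeginPlay stores the mesh's starting world rotation.
; A timeline plays forward to lerp the mesh's yaw up to 90 degrees from that start and reverses to close it.
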(event Custom|Open%20Door
  (bind _start_rotation (Variables|Default|GetStart%20Rotation))
  (bind (_roll _pitch _yaw) (Math|Rotator|BreakRotator _start_rotation))
  (bind _alpha (Timeline|OpenDoor Play)
    (:Update
      (Transformation|SetWorldRotation (Variables|Default|GetStaticMesh) (Math|Rotator|Lerp(Rotator) _start_rotation (Math|Rotator|MakeRotator _roll _pitch (+ _yaw 9e+01)) _alpha) false false))))

(event Custom|CloseDoor
  (bind _start_rotation (Variables|Default|GetStart%20Rotation))
  (bind (_roll _pitch _yaw) (Math|Rotator|BreakRotator _start_rotation))
  (bind _alpha (Timeline|OpenDoor Reverse)
    (:Update
      (Transformation|SetWorldRotation (Variables|Default|GetStaticMesh) (Math|Rotator|Lerp(Rotator) _start_rotation (Math|Rotator|MakeRotator _roll _pitch (+ _yaw 9e+01)) _alpha) false false))))

(event EventBeginPlay
  (Variables|Default|SetStart%20Rotation (Transformation|GetWorldRotation (Variables|Default|GetStaticMesh))))

(event Collision|EventActorBeginOverlap
  (params (OtherActor :type Actor%20Object%20Reference)))

(event EventTick
  (params (DeltaSeconds :type Float%20%28single-precision%29)))

(fn ConstructionScript)
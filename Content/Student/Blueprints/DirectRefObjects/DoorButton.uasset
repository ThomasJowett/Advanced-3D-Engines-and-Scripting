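; DoorButton is an interactable button actor that opens and closes a set of linked doors.
; Each Interact call alternates through a FlipFlop, calling OpenDoor or CloseDoor on every door in the DoorsToOpen array by direct reference.
; StartOutline and EndOutLine toggle custom depth rendering on its static mesh to show or hide an outline.
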(event EventBeginPlay)

(event Collision|EventActorBeginOverlap
  (params (OtherActor :type Actor%20Object%20Reference)))

(event EventTick
  (params (DeltaSeconds :type Float%20%28single-precision%29)))

(event EventStartOutline
  (Rendering|SetRenderCustomDepth (Variables|Default|GetStaticMesh) true))

(event EventEndOutLine
  (Rendering|SetRenderCustomDepth (Variables|Default|GetStaticMesh) false))

(event EventInteract
  (params (Interacted%20By :type Player%20Controller%20Object%20Reference))
  (bind _doorstoopen (Variables|Default|GetDoorsToOpen))
  (Utilities|FlowControl|FlipFlop
    (:A
      (for _array_element _doorstoopen
        (Default|OpenDoor _array_element)))
    (:B
      (for _array_element_2 _doorstoopen
        (Default|CloseDoor _array_element_2)))))

(fn ConstructionScript)
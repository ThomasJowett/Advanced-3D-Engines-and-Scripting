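; Minigun turret Blueprint that overrides FireWeapon to add hitscan shooting on top of its parent turret logic.
; Each shot line-traces along the Arrow's forward vector, applies point damage and spawns an emitter at the impact location, with the trace debug-drawn for the fire-rate duration.
; It also steps the Barrel's pitch via RInterpTo to spin it, then calls the parent FireWeapon.
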(event EventBeginPlay
  (|CallParentFunction))

(event Collision|EventActorBeginOverlap
  (params (OtherActor :type Actor%20Object%20Reference))
  (|CallParentFunction OtherActor))

(event EventTick
  (params (DeltaSeconds :type Float%20%28single-precision%29))
  (|CallParentFunction DeltaSeconds))

(fn ConstructionScript
  (|CallParentFunction))

(fn FireWeapon
  (params (Camera :type Camera%20Component%20Object%20Reference))
  (bind _arrow (Variables|Default|GetArrow))
  (bind _barrel (Variables|Default|GetBarrel))
  (bind _returnvalue (Math|Vector|GetForwardVector _arrow))
  (bind _returnvalue_2 (Transformation|GetWorldLocation _arrow))
  (bind _relativerotation (Variables|/Script/Engine.SceneComponent|GetRelativeRotation _barrel))
  (bind _returnvalue_3 (* _returnvalue 2e+05))
  (bind _outhit (Collision|LineTraceByChannel _returnvalue_2 (+ _returnvalue_2 _returnvalue_3) "TraceTypeQuery1" false 0 "ForDuration" true "(R=1.000000,G=0.000000,B=0.000000,A=1.000000)" "(R=0.000000,G=1.000000,B=0.000000,A=1.000000)" (Variables|Default|GetRateOfFire)))
  (Game|Damage|ApplyPointDamage (.HitActor (Collision|BreakHitResult _outhit)) (Variables|Default|GetDamage) _returnvalue_3 _outhit 0 self "/Engine/EngineDamageTypes/DmgTypeBP_Environmental.DmgTypeBP_Environmental_C")
  (Effects|SpawnEmitteratLocation 0 (.Location (Collision|BreakHitResult _outhit)))
  (Transformation|SetRelativeRotation _barrel (Math|Interpolation|RInterpTo (Math|Rotator|MakeRotator 0.0 (.pitch _relativerotation) 0.0) (Math|Rotator|MakeRotator 0.0 (+ (.pitch _relativerotation) 33.0) 0.0) (Variables|Default|GetDeltaTime) (Variables|Default|GetSpinSpeed)) false false)
  (bind _hasfired (|CallParentFunction 0))
  (return _hasfired))
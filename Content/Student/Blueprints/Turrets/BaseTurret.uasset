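; Base turret actor that targets the nearest enemy within attack range and reports team 0.
; Each tick it scans EnemyManagerRef's enemy list, yawing the holder toward the target and clamping gun pitch, or plays an idle timeline sweep.
; A looping rate-of-fire timer calls FireWeapon while the nearest distance is in range.
; The graph's EnemyManager lookup is unwired, so nothing here sets that reference.
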(event Custom|FireTurret
  ;[1 1 1] Begin Play
  (if (< (Variables|Default|GetDistance%20to%20Nearest%20Enemy) (Variables|Default|GetAttackRange)) ; Fire if in range
    (CallFunction|FireWeapon)))

(event EventBeginPlay
  ;[1 1 1] Begin Play
  (|CallParentFunction)
  (Utilities|Time|SetTimerbyEvent (delegate Custom|FireTurret) (Variables|Default|GetRateOfFire) true) ; Start the Firing Timer
  (Utilities|IsValid (Variables|Default|GetEnemy%20Manager%20Ref)))

(event EventTick
  (params (DeltaSeconds :type Float%20%28single-precision%29))
  ;[1 1 1] Find Ememy On Tick
  (bind _output_get (Variables|Default|SetDeltaTime DeltaSeconds))
  (|CallParentFunction _output_get)
  (bind _enemyfound (CallFunction|FindEnemy))
  (if _enemyfound ; If Enemy is Found then face them if not then play idle animation
    (Utilities|FlowControl|Sequence
      (:then_0
        ;[1 1 1] Idle Animation
        (bind _alpha (Timeline|Movement Stop)
          (:Update
            (Transformation|SetRelativeRotation (Variables|Default|GetTurret_Holder) (Math|Interpolation|RInterpTo (Variables|/Script/Engine.SceneComponent|GetRelativeRotation (Variables|Default|GetTurret_Holder)) (Math|Rotator|MakeRotator 0.0 0.0 (Math|Float|Lerp 6e+01 -6e+01 _alpha)) (Variables|Default|GetDeltaTime) (Variables|Default|GetRotationSpeed)) false false))))
      (:then_1
        (CallFunction|FaceEnemy)
        (Variables|Default|SetNearestEnemy 0)))
    (else
      (Timeline|Movement Play))))

(fn ConstructionScript
  (|CallParentFunction))

(fn FindEnemy
  (Variables|Default|SetDistance%20to%20Nearest%20Enemy (Variables|Default|GetAttackRange))
  (for _array_element (Variables|/Game/Student/Blueprints/Enemies/EnemyManager.EnemyManager_C|GetEnemies (Variables|Default|GetEnemy%20Manager%20Ref))
    (if (<= (Transformation|GetDistanceTo _array_element self) (Variables|Default|GetDistance%20to%20Nearest%20Enemy))
      (Variables|Default|SetDistance%20to%20Nearest%20Enemy (Transformation|GetDistanceTo _array_element self))
      (Variables|Default|SetNearestEnemy _array_element) ; Get the nearest
    ))
  (return (< (Variables|Default|GetDistance%20to%20Nearest%20Enemy) (Variables|Default|GetAttackRange))))

(fn FaceEnemy
  (bind _turret_holder (Variables|Default|GetTurret_Holder))
  (bind _nearestenemy (Variables|Default|GetNearestEnemy))
  (bind _arrow (Variables|Default|GetArrow))
  (bind _returnvalue (Transformation|GetWorldLocation _arrow))
  (bind _rootcomponent (Variables|/Script/Engine.Actor|GetRootComponent _nearestenemy))
  (bind _returnvalue_2 (Transformation|GetWorldLocation _rootcomponent))
  (bind _returnvalue_3 (Math|Rotator|FindLookatRotation _returnvalue _returnvalue_2))
  (Transformation|SetWorldRotation _turret_holder (Math|Interpolation|RInterpTo (Transformation|GetWorldRotation _turret_holder) (Math|Rotator|MakeRotator 0.0 0.0 (- (.yaw _returnvalue_3) 9e+01)) (Utilities|Time|GetWorldDeltaSeconds) (Variables|Default|GetRotationSpeed)) false false)
  (Transformation|SetRelativeRotation (Variables|Default|GetGun) (Math|Rotator|MakeRotator (Math|Float|ClampAngle (* (.pitch _returnvalue_3) -1.0) -3e+01 3e+01) 0.0 0.0) false false))

(fn GetTeam
  (return 0))
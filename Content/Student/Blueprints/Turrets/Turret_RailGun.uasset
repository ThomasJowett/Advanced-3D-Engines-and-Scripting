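; Railgun turret, a child of a turret base class that overrides FireWeapon to deal instant hitscan damage.
; After the parent call, it multi-line traces on Visibility along the Arrow's forward vector over a very long range.
; Every returned hit takes point damage equal to TurretDamage, using an environmental damage type.
; The trace is debug-drawn for the RateOfFire duration, and the function always returns true.
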(event EventBeginPlay
  (|CallParentFunction))

(event Collision|EventActorBeginOverlap
  (params (OtherActor :type Actor%20Object%20Reference))
  (|CallParentFunction OtherActor))

(event EventTick
  (params (DeltaSeconds :type Float%20%28single-precision%29))
  (|CallParentFunction DeltaSeconds))

(fn ConstructionScript
  (|CallParentFunction))

(fn FireWeapon
  (params (Camera :type Camera%20Component%20Object%20Reference))
  (bind _arrow (Variables|Default|GetArrow))
  (bind _returnvalue (Math|Vector|GetForwardVector _arrow))
  (bind _returnvalue_2 (Transformation|GetWorldLocation _arrow))
  (bind _returnvalue_3 (* _returnvalue 2e+05))
  (|CallParentFunction Camera)
  (bind _outhits (Collision|MultiLineTraceByChannel _returnvalue_2 (+ _returnvalue_2 _returnvalue_3) "TraceTypeQuery1" false 0 "ForDuration" true "(R=1.000000,G=0.000000,B=0.000000,A=1.000000)" "(R=0.000000,G=1.000000,B=0.000000,A=1.000000)" (Variables|Default|GetRateOfFire)))
  (for _array_element _outhits
    (Game|Damage|ApplyPointDamage (.HitActor (Collision|BreakHitResult _array_element)) (Variables|Default|GetTurretDamage) _returnvalue_3 _array_element 0 0 "/Engine/EngineDamageTypes/DmgTypeBP_Environmental.DmgTypeBP_Environmental_C"))
  (return true))
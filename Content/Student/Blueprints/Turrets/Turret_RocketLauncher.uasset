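; Rocket launcher turret, a child Blueprint that overrides its parent's FireWeapon to shoot rockets.
; FireWeapon spawns a RocketProjectile at the Gun's Rocket_1 socket, oriented by the Arrow component's world rotation, then calls the parent implementation and returns its result.
; The Camera input plays no part in aiming the spawn, and the event graph and construction script add no logic of their own.
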(event EventBeginPlay
  (|CallParentFunction))

(event Collision|EventActorBeginOverlap
  (params (OtherActor :type Actor%20Object%20Reference))
  (|CallParentFunction OtherActor))

(event EventTick
  (params (DeltaSeconds :type Float%20%28single-precision%29))
  (|CallParentFunction DeltaSeconds))

(fn ConstructionScript
  (|CallParentFunction))

(fn FireWeapon
  (params (Camera :type Camera%20Component%20Object%20Reference))
  (Game|SpawnActorfromClass "/Game/Student/Blueprints/Projectiles/RocketProjectile.RocketProjectile_C" (Math|Transform|MakeTransform (Transformation|GetSocketLocation (Variables|Default|GetGun) "Rocket_1") (Transformation|GetWorldRotation (Variables|Default|GetArrow))) "Undefined" 0 0)
  (bind _hasfired (|CallParentFunction 0))
  (return _hasfired))
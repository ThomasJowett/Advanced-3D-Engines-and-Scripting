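; Inventory component that holds a character's weight-limited item list and two weapon slots, equipped and back.
; Adding merges stackable items by ID; removing updates stack amounts and weight, with helpers for ammo and resource lookups.
; Items are used or dropped by spawning an actor from the item's ID class, with drops scattered randomly around the owner.
; Weapons attach, swap and drop with physics via message calls, and a slot index cycles the selected item.
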(fn AddItem
  (params (InventoryItem :type Inventory%20Item%20Structure))
  (bind (_id _icon _name _description _rarity _type _isstackable _worldmesh _damage _armour _health _amount _equippedmesh _ammotype _resourcetype _weight) (Utilities|Struct|BreakInventoryItem InventoryItem))
  (bind _inventory (Variables|Default|GetInventory))
  (if (<= (+ (* _amount _weight) (Variables|Default|GetCurrentWeight)) (Variables|Default|GetMaxWeight)) ; Is Inventory at max weight?
    (Variables|Default|SetCurrentWeight (+ (* _amount _weight) (Variables|Default|GetCurrentWeight)))
    (if _isstackable ; if the item stacks does a stack already exist
      (bind (_array_element _array_index) (Utilities|Array|ForEachLoopwithBreak _inventory :!label _label)
        (:LoopBody
          (if (== (.ID (Utilities|Struct|BreakInventoryItem _array_element)) _id)
            (LocalVariables|SetHasFoundItem true)
            (goto _label Break)))
        (:Completed
          (if (LocalVariables|GetHasFoundItem)
            (Utilities|Array|SetArrayElem _inventory _array_index (Utilities|Struct|MakeInventoryItem (.ID (Utilities|Struct|BreakInventoryItem _array_element)) (.Icon (Utilities|Struct|BreakInventoryItem _array_element)) (.Name (Utilities|Struct|BreakInventoryItem _array_element)) (.Description (Utilities|Struct|BreakInventoryItem _array_element)) (.Rarity (Utilities|Struct|BreakInventoryItem _array_element)) (.Type (Utilities|Struct|BreakInventoryItem _array_element)) (.IsStackable (Utilities|Struct|BreakInventoryItem _array_element)) (.WorldMesh (Utilities|Struct|BreakInventoryItem _array_element)) (.Damage (Utilities|Struct|BreakInventoryItem _array_element)) (.Armour (Utilities|Struct|BreakInventoryItem _array_element)) (.Health (Utilities|Struct|BreakInventoryItem _array_element)) (+ (.Amount (Utilities|Struct|BreakInventoryItem _array_element)) _amount) (.EquippedMesh (Utilities|Struct|BreakInventoryItem _array_element)) (.AmmoType (Utilities|Struct|BreakInventoryItem _array_element)) (.ResourceType (Utilities|Struct|BreakInventoryItem _array_element)) (.Weight (Utilities|Struct|BreakInventoryItem _array_element))))
            (else
              (Utilities|Array|Add _inventory InventoryItem :!label _label_2)))
          (return true)))
      (else
        (goto _label_2)))
    (else
      (Development|PrintString "Inventory Full")
      (return false))))

(fn RemoveItem
  (params (ItemToRemove :type Inventory%20Item%20Structure) (Ammount :type Integer))
  (bind _inventory (Variables|Default|GetInventory))
  (bind _returnvalue (Utilities|Array|FindItem _inventory ItemToRemove))
  (bind _output (Utilities|Array|Get(acopy) _inventory _returnvalue))
  (bind _amount (Utilities|Struct|BreakInventoryItem _output))
  (bind (_id _icon _name _description _rarity _type _isstackable _worldmesh _damage _armour _health _amount_2 _equippedmesh _ammotype _resourcetype _weight) (Utilities|Struct|BreakInventoryItem _output))
  (bind _returnvalue_2 (- _amount Ammount))
  (if (Utilities|Array|ContainsItem (Variables|Default|GetInventory) ItemToRemove)
    (if (<= _returnvalue_2 0)
      (Utilities|Array|RemoveItem (Variables|Default|GetInventory) _output)
      (Variables|Default|SetCurrentInventorySlot 0)
      (else
        (Utilities|Array|SetArrayElem _inventory _returnvalue (Utilities|Struct|MakeInventoryItem _id _icon _name _description _rarity _type _isstackable _worldmesh _damage _armour _health _returnvalue_2 _equippedmesh _ammotype _resourcetype _weight))))
    (Variables|Default|SetCurrentWeight (- (Variables|Default|GetCurrentWeight) (* Ammount (.Weight (Utilities|Struct|BreakInventoryItem ItemToRemove)))))
    (return true)
    (else
      (return false))))

(fn PickupWeapon
  (params (Weapon :type Base%20Player%20Weapon%20Object%20Reference))
  (bind _returnvalue (Components|GetOwner))
  (bind _ascharacter (Utilities|Casting|CastToCharacter _returnvalue))
  (Utilities|IsValid _ascharacter
    (:Is%20Valid
      (if (== (Variables|Default|GetEquippedWeapon) 0)
        (Class|WeaponsInterface|AttachtoPlayer(Message) Weapon _ascharacter)
        (elif (== (Variables|Default|GetBackWeapon) 0)
          (Class|WeaponsInterface|AttachtoPlayerBack(Message) Weapon _ascharacter)
          (else
            (return false))))
      (Variables|/Game/Student/Blueprints/PlayerWeapons/BasePlayerWeapon.BasePlayerWeapon_C|SetIsAttached Weapon true)
      (return true))
    (:Is%20Not%20Valid
      (Development|PrintString "Character Not Valid" true true "(R=1.000000,G=0.000000,B=0.000000,A=1.000000)"))))

(fn UseItem
  (params (UsedBy :type Actor%20Object%20Reference) (ItemUsed :type Inventory%20Item%20Structure))
  (bind _returnvalue (Game|SpawnActorfromClass (.ID (Utilities|Struct|BreakInventoryItem ItemUsed)) (Math|Transform|MakeTransform "0, 0, 0" "0, 0, 0" "1,1,1") "Undefined" 0 0))
  (Collision|SetActorEnableCollision _returnvalue false)
  (Transformation|AttachActorToActor _returnvalue (Components|GetOwner) "None" "KeepRelative" "KeepRelative" "KeepRelative" true)
  (bind _wasused (Class|InventoryInterface|UseItem(Message) _returnvalue))
  (if _wasused
    (bind _success (CallFunction|RemoveItem ItemUsed 1))
    (return _success)
    (else
      (Actor|DestroyActor _returnvalue)
      (return false))))

(fn DropWeapon
  (params (Weapon%20to%20Drop :type Base%20Player%20Weapon%20Object%20Reference))
  (Utilities|IsValid Weapon%20to%20Drop
    (:Is%20Valid
      (Transformation|DetachFromActor Weapon%20to%20Drop "KeepWorld" "KeepWorld" "KeepWorld")
      (Variables|/Game/Student/Blueprints/PlayerWeapons/BasePlayerWeapon.BasePlayerWeapon_C|SetIsAttached Weapon%20to%20Drop false)
      (Physics|SetEnableGravity (Variables|/Game/Student/Blueprints/PlayerWeapons/BasePlayerWeapon.BasePlayerWeapon_C|GetCapsule Weapon%20to%20Drop) true)
      (Physics|SetSimulatePhysics (Variables|/Game/Student/Blueprints/BaseWeapon.BaseWeapon_C|GetStaticMesh Weapon%20to%20Drop) true)
      (Variables|Default|SetEquippedWeapon 0)
      (Class|PlayerInterface|SwitchWeapon(Message) (Components|GetOwner)))))

(fn CycleEquipped
  (bind _returnvalue (Components|GetOwner))
  (bind _ascharacter (Utilities|Casting|CastToCharacter _returnvalue))
  (LocalVariables|SetTempWeaponRef (Variables|Default|GetEquippedWeapon))
  (Class|WeaponsInterface|AttachtoPlayer(Message) (Variables|Default|GetBackWeapon) _ascharacter)
  (Variables|Default|SetEquippedWeapon (Variables|Default|GetBackWeapon))
  (Class|WeaponsInterface|AttachtoPlayerBack(Message) (LocalVariables|GetTempWeaponRef) _ascharacter)
  (Variables|Default|SetBackWeapon (LocalVariables|GetTempWeaponRef)))

(fn DropItem
  (params (ItmeToDrop :type Inventory%20Item%20Structure) (Amount :type Integer))
  (bind _success (CallFunction|RemoveItem ItmeToDrop Amount))
  (if _success
    (bind _returnvalue (Game|SpawnActorfromClass (.ID (Utilities|Struct|BreakInventoryItem ItmeToDrop)) (Utilities|RandomLocationAroundCharacter) "Undefined" 0 0))
    (Class|InventoryInterface|DropItem(Message) _returnvalue ItmeToDrop (Components|GetOwner) Amount)))

(fn GetAmount
  (params (Item :type Inventory%20Item%20Structure))
  (bind _inventory (Variables|Default|GetInventory))
  (return (.Amount (Utilities|Struct|BreakInventoryItem (Utilities|Array|Get(acopy) _inventory (Utilities|Array|FindItem _inventory Item))))))

(fn GetAmountOfAmmo
  (params (AmmoType :type AmmoTypes%20Enum :default "NewEnumerator0"))
  (for (_array_element _array_index) (Variables|Default|GetInventory)
    (if (and (Utilities|Enum|Equal(Enum) (.Type (Utilities|Struct|BreakInventoryItem _array_element)) "NewEnumerator4") (Utilities|Enum|Equal(Enum) (.AmmoType (Utilities|Struct|BreakInventoryItem _array_element)) AmmoType))
      (return (.Amount (Utilities|Struct|BreakInventoryItem _array_element)) _array_index)))
  (return 0 0))

(fn GetAmountOfResource
  (params (PickUpType :type ResourceTypes%20Enum :default "NewEnumerator0"))
  (for (_array_element _array_index) (Variables|Default|GetInventory)
    (if (and (Utilities|Enum|Equal(Enum) (.Type (Utilities|Struct|BreakInventoryItem _array_element)) "NewEnumerator3") (Utilities|Enum|Equal(Enum) (.ResourceType (Utilities|Struct|BreakInventoryItem _array_element)) PickUpType))
      (return (.Amount (Utilities|Struct|BreakInventoryItem _array_element)) _array_index)))
  (return 0 0))

(fn RemoveResource
  (params (ResourceType :type ResourceTypes%20Enum :default "NewEnumerator0") (Amount :type Integer))
  (for _array_element (Variables|Default|GetInventory)
    (if (Utilities|Enum|Equal(Enum) (.ResourceType (Utilities|Struct|BreakInventoryItem _array_element)) ResourceType)
      (bind _success (CallFunction|RemoveItem _array_element Amount))
      (return _success)))
  (return false))

(fn NextItem
  (bind _result (Math|Integer|IncrementInt (Variables|Default|GetCurrentInventorySlot))
    (:%20%20
      (if (> _result (- (Utilities|Array|Length (Variables|Default|GetInventory)) 1))
        (Variables|Default|SetCurrentInventorySlot 0)))))

(fn PreviousItem
  (bind _result (Math|Integer|DecrementInt (Variables|Default|GetCurrentInventorySlot))
    (:%20%20
      (if (< _result 0)
        (Variables|Default|SetCurrentInventorySlot (- (Utilities|Array|Length (Variables|Default|GetInventory)) 1))))))

(fn DropCurrentItem
  (bind _inventory (Variables|Default|GetInventory))
  (bind _currentinventoryslot (Variables|Default|GetCurrentInventorySlot))
  (bind _output (Utilities|Array|Get(acopy) _inventory _currentinventoryslot))
  (if (> (Utilities|Array|Length _inventory) 0)
    (bind _amount (CallFunction|GetAmount _output))
    (CallFunction|DropItem _output _amount)))

(fn UseCurrentItem
  (bind _inventory (Variables|Default|GetInventory))
  (if (> (Utilities|Array|Length _inventory) 0)
    (CallFunction|UseItem (Components|GetOwner) (Utilities|Array|Get(acopy) _inventory (Variables|Default|GetCurrentInventorySlot)))))

(fn AddResource
  (params (ResourceType :type ResourceTypes%20Enum :default "NewEnumerator0") (Ammount :type Integer))
  (for _array_element (Variables|Default|GetInventory)
    (if (Utilities|Enum|Equal(Enum) (.ResourceType (Utilities|Struct|BreakInventoryItem _array_element)) ResourceType)
      (bind _success (CallFunction|AddItem (Utilities|Struct|MakeInventoryItem (.ID (Utilities|Struct|BreakInventoryItem _array_element)) (.Icon (Utilities|Struct|BreakInventoryItem _array_element)) (.Name (Utilities|Struct|BreakInventoryItem _array_element)) (.Description (Utilities|Struct|BreakInventoryItem _array_element)) (.Rarity (Utilities|Struct|BreakInventoryItem _array_element)) (.Type (Utilities|Struct|BreakInventoryItem _array_element)) (.IsStackable (Utilities|Struct|BreakInventoryItem _array_element)) (.WorldMesh (Utilities|Struct|BreakInventoryItem _array_element)) (.Damage (Utilities|Struct|BreakInventoryItem _array_element)) (.Armour (Utilities|Struct|BreakInventoryItem _array_element)) (.Health (Utilities|Struct|BreakInventoryItem _array_element)) Ammount (.EquippedMesh (Utilities|Struct|BreakInventoryItem _array_element)) (.AmmoType (Utilities|Struct|BreakInventoryItem _array_element)) (.ResourceType (Utilities|Struct|BreakInventoryItem _array_element)) (.Weight (Utilities|Struct|BreakInventoryItem _array_element)))))
      (return _success)))
  (return false))
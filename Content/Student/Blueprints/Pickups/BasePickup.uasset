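; Base world pickup actor for items, driven by an ItemInfo struct that sets its mesh and destroyed automatically after LifeTime.
; PickupItem passes itself and ItemInfo to the picker through PickUpMessage, then destroys the actor.
; Outline events toggle custom depth, with the stencil value derived from item rarity at construction.
; DropItem rebuilds ItemInfo with the dropped amount, while UseItem is a stub returning false.
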(event Custom|UseItem_1_1)

(event EventBeginPlay
  (Utilities|FlowControl|Delay (Variables|Default|GetLifeTime))
  (Actor|DestroyActor))

(event Collision|EventActorBeginOverlap
  (params (OtherActor :type Actor%20Object%20Reference)))

(event EventDropItem
  (params (Dropped%20Item :type Inventory%20Item%20Structure) (Dropped%20By :type Actor%20Object%20Reference) (AmountDropped :type Integer))
  (Variables|Default|SetItemInfo (Utilities|Struct|MakeInventoryItem (.id (Variables|Default|GetItemInfo)) (.icon (Variables|Default|GetItemInfo)) (.name (Variables|Default|GetItemInfo)) (.description (Variables|Default|GetItemInfo)) (.rarity (Variables|Default|GetItemInfo)) (.type (Variables|Default|GetItemInfo)) (.isstackable (Variables|Default|GetItemInfo)) (.worldmesh (Variables|Default|GetItemInfo)) (.damage (Variables|Default|GetItemInfo)) (.armour (Variables|Default|GetItemInfo)) (.health (Variables|Default|GetItemInfo)) AmountDropped (.equippedmesh (Variables|Default|GetItemInfo)) (.ammotype (Variables|Default|GetItemInfo)) (.resourcetype (Variables|Default|GetItemInfo)) (.weight (Variables|Default|GetItemInfo)))))

(event EventTick
  (params (DeltaSeconds :type Float%20%28single-precision%29)))

(event EventStartOutline
  ;[1 1 1] Outlines
  (Rendering|SetRenderCustomDepth (Variables|Default|GetStaticMesh) true))

(event EventEndOutLine
  ;[1 1 1] Outlines
  (Rendering|SetRenderCustomDepth (Variables|Default|GetStaticMesh) false))

(event EventPickupItem
  (params (PickedUpBy :type Actor%20Object%20Reference) (ItemPickedUp :type Actor%20Object%20Reference))
  ;[1 1 1] Gets picked up by player
  (Class|PlayerInterface|PickUp(Message) PickedUpBy self (Variables|Default|GetItemInfo))
  (Actor|DestroyActor))

(fn ConstructionScript
  (bind _iteminfo (Variables|Default|GetItemInfo))
  (bind _staticmesh (Variables|Default|GetStaticMesh))
  (bind (_id _icon _name _description _rarity _type _isstackable _worldmesh) (Utilities|Struct|BreakInventoryItem _iteminfo))
  (Components|StaticMesh|SetStaticMesh _staticmesh _worldmesh)
  (Rendering|SetCustomDepthStencilValue _staticmesh (+ (Math|Conversions|ToInteger(Byte) _rarity) 1)))

(fn GetItemInfo
  (return (Variables|Default|GetItemInfo)))

(fn UseItem
  (return false))
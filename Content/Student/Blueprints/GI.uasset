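; Game Instance Blueprint that tracks the main game state and handles level travel, loading screen and quitting.
; Init sets the state to StartUp, and UpdateMainGameState changes it on request.
; Start and exit act only from Main Menu, while returning to the menu map works from Loading Screen, Playing or Playing Paused.
; Separate events create and remove the loading screen widget, independent of state.
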(event Custom|TriggerLoadingScreen
  (bind _returnvalue (UserInterface|CreateWidget "/Game/Student/UI/LoadingScreen.LoadingScreen_C"))
  (bind _output_get (Variables|Default|SetLoading%20Screen%20Widget _returnvalue))
  (UserInterface|Viewport|AddtoViewport _output_get 0))

(event Custom|ExitGame
  (switch Utilities|FlowControl|Switch|SwitchonMainGameStates (Variables|Default|GetCurrentState)
    (:NewEnumerator1
      (Game|QuitGame 0 "Quit"))))

(event Custom|ReturnToMainMenu
  (switch Utilities|FlowControl|Switch|SwitchonMainGameStates (Variables|Default|GetCurrentState)
    (:NewEnumerator2
      _)
    (:NewEnumerator3
      _)
    (:NewEnumerator4
      _))
  (Game|OpenLevel(byName) "MenuScreen"))

(event Custom|TriggerLoadingScreenDestruction
  (bind _loading_screen_widget (Variables|Default|GetLoading%20Screen%20Widget))
  (Utilities|IsValid _loading_screen_widget
    (:Is%20Valid
      (Widget|RemovefromParent _loading_screen_widget))))

(event Custom|UpdateMainGameState
  (params (GameState :type MainGameStates%20Enum :default "NewEnumerator0"))
  (Variables|Default|SetCurrentState GameState))

(event Custom|StartLevel
  (switch Utilities|FlowControl|Switch|SwitchonMainGameStates (Variables|Default|GetCurrentState)
    (:NewEnumerator1
      (Game|OpenLevel(byName) "ThirdPersonExampleMap"))))

(event EventInit
  (Variables|Default|SetCurrentState "NewEnumerator0"))
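; Game mode that respawns the player and keeps a list of living enemies.
; On BeginPlay it binds to the player character's destroyed event and caches all PlayerStart and EnemyCharacter actors.
; When the character is destroyed, it restarts the player at the first cached PlayerStart and binds to the new character.
; The Died event removes the given enemy from the list.
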(event Custom|Respawn
  ;[1 1 1] Character Death
  (Game|BindEventtoOnDestroyed (Game|GetPlayerCharacter 0) (delegate Custom|Event%20Destroyed)))

(event Custom|Event%20Destroyed
  (params (DestroyedActor :type Actor%20Object%20Reference))
  ;[1 1 1] Character Death
  (Class|GameModeBase|RestartPlayeratPlayerStart (Game|GetPlayerController 0) (Utilities|Array|Get(acopy) (Variables|Default|GetPlayerStarts)))
  (CallFunction|Respawn))

(event EventBeginPlay
  (CallFunction|Respawn)
  (bind _outactors (Actor|GetAllActorsOfClass "/Script/Engine.PlayerStart"))
  (Variables|Default|SetPlayerStarts _outactors)
  (bind _outactors_2 (Actor|GetAllActorsOfClass "/Game/Student/Blueprints/Enemies/EnemyCharacter.EnemyCharacter_C"))
  (Variables|Default|SetAllEnemies _outactors_2))

(event EventDied
  (params (Enemy :type Actor%20Object%20Reference))
  (Utilities|Array|RemoveItem (Variables|Default|GetAllEnemies) Enemy))

(fn ConstructionScript)
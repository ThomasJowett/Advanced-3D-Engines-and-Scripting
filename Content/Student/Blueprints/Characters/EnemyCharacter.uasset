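; AI enemy character that fights with a shotgun and drops random pickups when killed.
; On BeginPlay it rolls a random loot list and attaches a spawned, loaded, collision-free shotgun.
; AI perception of non-enemy MyCharacters updates Blackboard target and visibility keys, while Attack fires the equipped weapon.
; Death notifies the game mode, scatters the loot pickups around the body, then destroys the actor after a short delay.
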(event OnTargetPerceptionUpdated(AIPerception)
  (params (Actor :type Actor%20Object%20Reference) (Stimulus :type AI%20Stimulus%20Structure))
  (bind _returnvalue (AI|GetBlackboard 0))
  (bind _asmy_character (Utilities|Casting|CastToMyCharacter Actor))
  (Utilities|Casting|CastToEnemyCharacter Actor
    (:CastFailed
      (AI|Components|Blackboard|SetValueasBool _returnvalue (Utilities|Name|MakeLiteralName "Can See Player") (.bSuccessfullySensed (Utilities|Struct|BreakAIStimulus Stimulus)))
      (AI|Components|Blackboard|SetValueasObject _returnvalue (Utilities|Name|MakeLiteralName "Player") _asmy_character))))

(event EventBeginPlay
  (|CallParentFunction)
  (CallFunction|GenerateLoot)
  (bind _returnvalue (Game|SpawnActorfromClass "/Game/Student/Blueprints/PlayerWeapons/ShotGun.ShotGun_C" (Math|Transform|MakeTransform "0, 0, 0" "0, 0, 0" "1,1,1") "Undefined" 0 0))
  (Class|WeaponsInterface|AttachtoPlayer(Message) _returnvalue self)
  (Variables|/Game/Student/Blueprints/PlayerWeapons/BasePlayerWeapon.BasePlayerWeapon_C|SetCurrentAmmoLoaded _returnvalue 100)
  (Collision|SetActorEnableCollision _returnvalue false))

(event EventDie
  (|CallParentFunction)
  (Class|EnemyInterface|Died(Message) (Game|GetGameMode) self)
  (CallFunction|DropLoot)
  (Utilities|FlowControl|Delay 2.0)
  (Actor|DestroyActor))

(event EventAttack
  (Class|WeaponsInterface|FireWeapon(Message) (Variables|/Game/Student/Blueprints/Inventory/InventoryComponent.InventoryComponent_C|GetEquippedWeapon (Variables|Default|GetInventoryComponent)) (Variables|Default|GetThirdPersonCamera)))

(fn ConstructionScript
  (|CallParentFunction))

(fn DropLoot
  (bind _self self)
  (bind _location (Utilities|GetLocationAroundActor _self 64.0 96.0))
  (for _array_element (Variables|Default|GetResourcesToDrop)
    (switch Utilities|FlowControl|Switch|SwitchonPickUpTypes _array_element
      (:NewEnumerator0
        (Game|SpawnActorfromClass "/Game/Student/Blueprints/Pickups/GrenadesPickup.GrenadesPickup_C" _location "Undefined" 0 0))
      (:NewEnumerator1
        (Game|SpawnActorfromClass "/Game/Student/Blueprints/Pickups/BulletsPickup.BulletsPickup_C" _location "Undefined" 0 0))
      (:NewEnumerator2
        (Game|SpawnActorfromClass "/Game/Student/Blueprints/Pickups/SpringsPickup.SpringsPickup_C" _location "Undefined" 0 0))
      (:NewEnumerator3
        (Game|SpawnActorfromClass "/Game/Student/Blueprints/Pickups/MetalSheetsPickup.MetalSheetsPickup_C" _location "Undefined" 0 0))
      (:NewEnumerator4
        (Game|SpawnActorfromClass "/Game/Student/Blueprints/Pickups/PipesPickup.PipesPickup_C" _location "Undefined" 0 0))
      (:NewEnumerator5
        (Game|SpawnActorfromClass "/Game/Student/Blueprints/Pickups/HealthPickup.HealthPickup_C" _location "Undefined" 0 0)))))

(fn GenerateLoot
  (for _index (range 0 (Math|Random|RandomIntegerinRange 0 5))
    (Utilities|Array|Add (Variables|Default|GetResourcesToDrop) (Utilities|Enum|ByteToEnumPickUpTypes (Math|Conversions|ToByte(Integer) (Math|Random|RandomIntegerinRange 0 (- (|GetNumEnumEntries) 1)))))))
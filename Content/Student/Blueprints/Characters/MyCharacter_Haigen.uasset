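; MyCharacter_Haigen is a character Blueprint that arms itself when play begins.
; On BeginPlay it runs the parent logic, spawns a shotgun at the origin and messages it to attach to the character.
; It then spawns a bullets pickup, adds its item info to the InventoryComponent, and sends it a pickup message with the character's controller as collector.
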(event EventBeginPlay
  (bind _returnvalue (Math|Transform|MakeTransform "0, 0, 0"))
  (|CallParentFunction)
  (bind _returnvalue_2 (Game|SpawnActorfromClass "/Game/Student/Blueprints/PlayerWeapons/ShotGun.ShotGun_C" _returnvalue "Undefined" 0 0))
  (Class|WeaponsInterface|AttachtoPlayer(Message) _returnvalue_2 self)
  (bind _returnvalue_3 (Game|SpawnActorfromClass "/Game/Student/Blueprints/Pickups/BulletsPickup.BulletsPickup_C" _returnvalue "Undefined" 0 0))
  (Default|AddItem (Variables|Default|GetInventoryComponent) (Variables|/Game/Student/Blueprints/Pickups/BasePickup.BasePickup_C|GetItemInfo _returnvalue_3))
  (Class|InventoryInterface|PickupItem(Message) _returnvalue_3 (Pawn|GetController) _returnvalue_3))

(fn ConstructionScript
  (|CallParentFunction))
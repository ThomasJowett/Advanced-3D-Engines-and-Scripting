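; Player-controller component for building mode that previews and places turrets, blocks, ramps and enemy spawners.
; Selecting an item spawns a hologram, tinted by whether the pawn's inventory covers its resource cost, and cycling skips Spawner outside Versus mode.
; The hologram snaps to a grid and 90-degree yaw, with short vertical traces hiding it and blocking placement when nothing is hit.
; Building spawns the real actor, wires in team manager references and deducts resources.
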(event EventBeginPlay
  (CallFunction|SetBuildItem "NewEnumerator3" "Forward"))

(event EventTick
  (params (DeltaSeconds :type Float%20%28single-precision%29)))

(event EventSetLocation
  (params (Location :type Vector :default "0, 0, 0"))
  (CallFunction|SetBuildLocation Location))

(event EventSetBuildItem
  (params (ItemToBuild :type BuildItems%20Enum :default "NewEnumerator0"))
  (CallFunction|SetBuildItem ItemToBuild "Forward"))

(event EventBuild
  (CallFunction|BuildItem))

(fn HideActor
  (bind _itemref (Variables|Default|GetItemRef))
  (Utilities|IsValid _itemref
    (:Is%20Valid
      (Transformation|SetActorLocation _itemref "0, 0,-100.000000" false true)
      (Variables|Default|SetItemCanBeBuilt false))))

(fn BuildItem
  (bind _actortransform (Variables|Default|GetActorTransform))
  (if (and (Variables|Default|GetItemCanBeBuilt) (Variables|Default|GetCanAffordItem))
    (bind _returnvalue (Class|GameplayStatics|GetPlayerControllerID (.AsPlayer%20Controller (Utilities|Casting|CastToPlayerController (Components|GetOwner)))))
    (bind _enemymanager (Class|GameModeInterface|GetEnemyManager(Message) (Game|GetGameMode) _returnvalue))
    (switch Utilities|FlowControl|Switch|SwitchonBuildItems (Variables|Default|GetItemID)
      (:NewEnumerator0
        (bind _returnvalue_2 (Game|SpawnActorfromClass "/Game/Student/Blueprints/Turrets/Turret_MiniGun.Turret_MiniGun_C" _actortransform "Undefined" 0 _enemymanager 0))
        (CallFunction|RemoveResources)
        (return _returnvalue_2))
      (:NewEnumerator1
        (bind _returnvalue_3 (Game|SpawnActorfromClass "/Game/Student/Blueprints/Turrets/Turret_RocketLauncher.Turret_RocketLauncher_C" _actortransform "Undefined" 0 _enemymanager 0))
        (CallFunction|RemoveResources)
        (return _returnvalue_3))
      (:NewEnumerator2
        (bind _returnvalue_4 (Game|SpawnActorfromClass "/Game/Student/Blueprints/Turrets/Turret_RailGun.Turret_RailGun_C" _actortransform "Undefined" 0 _enemymanager 0))
        (CallFunction|RemoveResources)
        (return _returnvalue_4))
      (:NewEnumerator3
        (bind _returnvalue_5 (Game|SpawnActorfromClass "/Game/Student/Blueprints/Building/Block.Block_C" _actortransform "Undefined" 0 0))
        (CallFunction|RemoveResources)
        (return _returnvalue_5))
      (:NewEnumerator4
        (bind _returnvalue_6 (Game|SpawnActorfromClass "/Game/Student/Blueprints/Building/Ramp.Ramp_C" _actortransform "Undefined" 0 0))
        (CallFunction|RemoveResources)
        (return _returnvalue_6))
      (:NewEnumerator5
        (bind _core (Class|GameModeInterface|GetCore(Message) (Game|GetGameMode) _returnvalue))
        (bind _returnvalue_7 (Game|SpawnActorfromClass "/Game/Student/Blueprints/Enemies/EnemySpawnPoint.EnemySpawnPoint_C" _actortransform "Undefined" 0 _core _enemymanager -1 0))
        (CallFunction|RemoveResources)
        (return _returnvalue_7)))))

(fn SetBuildItem
  (params (ItemID :type BuildItems%20Enum :default "NewEnumerator0") (Direction :type ETimelineDirection%20Enum :default "Forward"))
  (bind _actortransform (Variables|Default|GetActorTransform))
  (Utilities|IsValid (Variables|Default|GetItemRef)
    (:Is%20Valid
      (Actor|DestroyActor (Variables|Default|GetItemRef)))
    (:Is%20Not%20Valid
      _))
  (bind _output_get (Variables|Default|SetItemID ItemID))
  (switch Utilities|FlowControl|Switch|SwitchonBuildItems _output_get
    (:NewEnumerator0
      (bind _returnvalue (Game|SpawnActorfromClass "/Game/Student/Blueprints/Building/HologramMiniGun.HologramMiniGun_C" _actortransform "Undefined" 0 0))
      (Variables|Default|SetItemRef _returnvalue)
      (bind _hasenough (CallFunction|HasEnoughResources _returnvalue))
      (CallFunction|SetMaterial _hasenough))
    (:NewEnumerator1
      (bind _returnvalue_2 (Game|SpawnActorfromClass "/Game/Student/Blueprints/Building/HologramRocketLauncher.HologramRocketLauncher_C" _actortransform "Undefined" 0 0))
      (Variables|Default|SetItemRef _returnvalue_2)
      (bind _hasenough_2 (CallFunction|HasEnoughResources _returnvalue_2))
      (CallFunction|SetMaterial _hasenough_2))
    (:NewEnumerator2
      (bind _returnvalue_3 (Game|SpawnActorfromClass "/Game/Student/Blueprints/Building/HologramRailGun.HologramRailGun_C" _actortransform "Undefined" 0 0))
      (Variables|Default|SetItemRef _returnvalue_3)
      (bind _hasenough_3 (CallFunction|HasEnoughResources _returnvalue_3))
      (CallFunction|SetMaterial _hasenough_3))
    (:NewEnumerator3
      (bind _returnvalue_4 (Game|SpawnActorfromClass "/Game/Student/Blueprints/Building/HologramBlock.HologramBlock_C" _actortransform "Undefined" 0 0))
      (Variables|Default|SetItemRef _returnvalue_4)
      (bind _hasenough_4 (CallFunction|HasEnoughResources _returnvalue_4))
      (CallFunction|SetMaterial _hasenough_4))
    (:NewEnumerator4
      (bind _returnvalue_5 (Game|SpawnActorfromClass "/Game/Student/Blueprints/Building/HologramRamp.HologramRamp_C" _actortransform "Undefined" 0 0))
      (Variables|Default|SetItemRef _returnvalue_5)
      (bind _hasenough_5 (CallFunction|HasEnoughResources _returnvalue_5))
      (CallFunction|SetMaterial _hasenough_5))
    (:NewEnumerator5
      (bind _asmy_game_instance (Utilities|Casting|CastToMyGameInstance (Game|GetGameInstance)))
      (switch Utilities|FlowControl|Switch|SwitchonGameModes (Variables|/Game/Student/Blueprints/MyGameInstance.MyGameInstance_C|GetGameMode _asmy_game_instance)
        (:NewEnumerator0
          (switch Utilities|FlowControl|Switch|SwitchonETimelineDirection Direction :!label _label
            (:Forward
              (CallFunction|NextBuildItem))
            (:Backward
              (CallFunction|PreviousBuildItem))))
        (:NewEnumerator1
          (bind _returnvalue_6 (Game|SpawnActorfromClass "/Game/Student/Blueprints/Building/HologramEnemySpawner.HologramEnemySpawner_C" _actortransform "Undefined" 0 0))
          (Variables|Default|SetItemRef _returnvalue_6)
          (bind _hasenough_6 (CallFunction|HasEnoughResources _returnvalue_6))
          (CallFunction|SetMaterial _hasenough_6))
        (:NewEnumerator2
          (goto _label))))))

(fn SetBuildLocation
  (params (Location :type Vector))
  (bind (_x _y _z) (Math|Vector|BreakVector Location))
  (bind _itemref (Variables|Default|GetItemRef))
  (bind _grid_spacing (Variables|Default|GetGrid%20Spacing))
  (bind _itemref_2 (Variables|Default|GetItemRef))
  (bind _grid_spacing_2 (Variables|Default|GetGrid%20Spacing))
  (bind _itemref_3 (Variables|Default|GetItemRef))
  (bind _returnvalue (Transformation|GetActorLocation _itemref_2))
  (bind _returnvalue_2 (Transformation|GetActorLocation _itemref))
  (bind (_x_2 _y_2 _z_2) (Math|Vector|BreakVector _returnvalue))
  (bind (_x_3 _y_3 _z_3) (Math|Vector|BreakVector _returnvalue_2))
  (Variables|Default|SetActorTransform (Math|Transform|MakeTransform (Math|Vector|MakeVector (* (Math|Float|Round (/ _x _grid_spacing_2)) _grid_spacing) (* (Math|Float|Round (/ _y _grid_spacing_2)) _grid_spacing) _z) (Math|Rotator|MakeRotator 0.0 0.0 (+ (* (Math|Float|Round (/ (.yaw (Transformation|GetActorRotation (Components|GetOwner))) 9e+01)) 9e+01) 9e+01)) "1,1,1"))
  (Utilities|IsValid _itemref_3
    (:Is%20Valid
      (Transformation|SetActorTransform _itemref_3 (Variables|Default|GetActorTransform))
      (bind _returnvalue_3 (Collision|LineTraceByChannel _returnvalue_2 (Math|Vector|MakeVector _x_3 _y_3 (- _z_3 1e+01)) "TraceTypeQuery1" false 0 "None"))
      (bind _returnvalue_4 (Collision|LineTraceByChannel "0, 0, 0" (Math|Vector|MakeVector _x_2 _y_2 (+ _z_2 1e+01)) "TraceTypeQuery1" false 0 "None"))
      (if (or _returnvalue_3 _returnvalue_4)
        (Variables|Default|SetItemCanBeBuilt true)
        (else
          (CallFunction|HideActor))))))

(fn SetMaterial
  (params (CanBuild :type Boolean))
  (Class|BuildObjectInterface|SetCanBuildMaterial(Message) (Variables|Default|GetItemRef) CanBuild))

(fn NextBuildItem
  (bind _itemid (Variables|Default|GetItemID))
  (bind _returnvalue (Math|Conversions|ToInteger(Byte) _itemid))
  (bind _returnvalue_2 (+ _returnvalue 1))
  (if (> _returnvalue_2 (- (|GetNumEnumEntries) 1))
    (CallFunction|SetBuildItem (Utilities|Enum|ByteToEnumBuildItems (Math|Conversions|ToByte(Integer) 0)) "Forward")
    (else
      (CallFunction|SetBuildItem (Utilities|Enum|ByteToEnumBuildItems (Math|Conversions|ToByte(Integer) _returnvalue_2)) "Forward"))))

(fn PreviousBuildItem
  (bind _itemid (Variables|Default|GetItemID))
  (bind _returnvalue (Math|Conversions|ToInteger(Byte) _itemid))
  (bind _returnvalue_2 (- _returnvalue 1))
  (if (< _returnvalue_2 0)
    (CallFunction|SetBuildItem (Utilities|Enum|ByteToEnumBuildItems (Math|Conversions|ToByte(Integer) (- (|GetNumEnumEntries) 1))) "Backward")
    (else
      (CallFunction|SetBuildItem (Utilities|Enum|ByteToEnumBuildItems (Math|Conversions|ToByte(Integer) _returnvalue_2)) "Backward"))))

(fn HasEnoughResources
  (params (Hologram :type Hologram%20Build%20Object%20Object%20Reference))
  (bind _controlledpawn (Class|PlayerControllerInterface|GetControlledPawn(Message) (Components|GetOwner)))
  (bind _inventorycomponent (Class|CharacterInterface|ReturnInventoryComponent(Message) _controlledpawn))
  (Utilities|IsValid _inventorycomponent
    (:Is%20Valid
      (bind _array_element (Utilities|Array|ForEachLoopwithBreak (Variables|/Game/Student/Blueprints/Building/HologramBuildObject.HologramBuildObject_C|GetResourcesNeeded Hologram))
        (:LoopBody
          (bind _amount (Default|GetAmountOfResource _inventorycomponent (.ResourceType (Utilities|Struct|BreakResourcesNeeded _array_element))))
          (if (not (>= _amount (.Ammount (Utilities|Struct|BreakResourcesNeeded _array_element))))
            (Variables|Default|SetCanAffordItem false)
            (return false)))
        (:Completed
          (Variables|Default|SetCanAffordItem true)
          (return true))))
    (:Is%20Not%20Valid
      (Variables|Default|SetCanAffordItem false)
      (return false))))

(fn RemoveResources
  (bind _itemref (Variables|Default|GetItemRef))
  (bind _controlledpawn (Class|PlayerControllerInterface|GetControlledPawn(Message) (Components|GetOwner)))
  (bind _inventorycomponent (Class|CharacterInterface|ReturnInventoryComponent(Message) _controlledpawn))
  (Utilities|IsValid _inventorycomponent
    (:Is%20Valid
      (for _array_element (Variables|/Game/Student/Blueprints/Building/HologramBuildObject.HologramBuildObject_C|GetResourcesNeeded _itemref)
        (Default|RemoveResource _inventorycomponent (.ResourceType (Utilities|Struct|BreakResourcesNeeded _array_element)) (.Ammount (Utilities|Struct|BreakResourcesNeeded _array_element))))
      (bind _hasenough (CallFunction|HasEnoughResources _itemref))
      (CallFunction|SetMaterial _hasenough))))

(fn ReturnResources
  (bind _controlledpawn (Class|PlayerControllerInterface|GetControlledPawn(Message) (Components|GetOwner)))
  (bind _inventorycomponent (Class|CharacterInterface|ReturnInventoryComponent(Message) _controlledpawn))
  (Utilities|IsValid _inventorycomponent
    (:Is%20Valid
      (for _array_element (Variables|/Game/Student/Blueprints/Building/HologramBuildObject.HologramBuildObject_C|GetResourcesNeeded (Variables|Default|GetItemRef))
        (Default|AddResource _inventorycomponent (.ResourceType (Utilities|Struct|BreakResourcesNeeded _array_element)) (.Ammount (Utilities|Struct|BreakResourcesNeeded _array_element)))))))
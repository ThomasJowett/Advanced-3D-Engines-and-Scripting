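; Hologram preview actor for a buildable turret-like object made of Base, Holder, Gun and Barrel meshes.
; The construction script applies the BuildHologram material to the first two material slots of every part.
; SetCanBuildMaterial switches the CanBuild scalar parameter on all parts to show whether placement is valid, and prints a debug message for each state.
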(event EventBeginPlay)

(event Collision|EventActorBeginOverlap
  (params (OtherActor :type Actor%20Object%20Reference)))

(event EventTick
  (params (DeltaSeconds :type Float%20%28single-precision%29)))

(event EventSetCanBuildMaterial
  (params (CanBuild :type Boolean))
  (bind _barrel (Variables|Default|GetBarrel))
  (if CanBuild
    (Rendering|Material|SetScalarParameterValueonMaterials _barrel "CanBuild" 0.0)
    (Development|PrintString "CanBuild")
    (else
      (Rendering|Material|SetScalarParameterValueonMaterials _barrel "CanBuild" 1.0)
      (Development|PrintString "CanNotBuild" true true "(R=1.000000,G=0.064041,B=0.000000,A=1.000000)"))))

(fn ConstructionScript
  (Rendering|Material|SetMaterial (Variables|Default|GetBase) 0 "/Game/Student/Assets/Materials/BuildHologram.BuildHologram")
  (Rendering|Material|SetMaterial (Variables|Default|GetBarrel) 1 "/Game/Student/Assets/Materials/BuildHologram.BuildHologram"))